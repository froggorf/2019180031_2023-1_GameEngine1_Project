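; Board-game GameMode that runs each player's turn through item select, item use, dice, move and board-action steps.
; Tick dispatches on the GameStepString state for two players, with DoOnce gates for step entry and finish events advancing it.
; Items alter the roll or warp via pipe, and bought stars respawn on another random StarBoard.
; It drives camera, input mappings and GameState UI; the minigame step just restarts at player 0.
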(event Custom|Finish%20Item%20Select
  ;[1 1 1] PLAYER_ITEM
  (bind _asgs_board_game (Utilities|Casting|CastToGS_BoardGame (Game|GetGameState)))
  (Default|ItemUIHidden _asgs_board_game)
  (Variables|Default|SetGame%20Step%20String (Utilities|String|Append "PLAYER" (Utilities|String|ToString(Integer) (Variables|/Game/BoardGame/Character/BP_BoardCharacter.BP_BoardCharacter_C|GetPlayerNumber (stale Custom|PLAYER_ITEM Player))) "_ITEMUSING"))
  (Utilities|FlowControl|DoOnce false) ; enters at Reset
)

(event Custom|Using%20Pipe
  (params (Pipe%20Using%20Player :type BP%20Board%20Character%20Object%20Reference))
  ;[1 1 1] ITEMUSING Pipe Logic
  (Utilities|FlowControl|DoOnce false
    (:Completed
      (bind _asgs_board_game (Utilities|Casting|CastToGS_BoardGame (Game|GetGameState)))
      (Default|SetTargetActor (Variables|Default|GetMain%20Camera) (Utilities|Array|Get(acopy) (Variables|/Game/BoardGame/Core/GS_BoardGame.GS_BoardGame_C|GetBoards _asgs_board_game) (Math|Integer|%(Integer) (+ (Variables|/Game/BoardGame/Character/BP_BoardCharacter.BP_BoardCharacter_C|GetCurrent%20Board%20Number Pipe%20Using%20Player) 1) (Utilities|Array|Length (Variables|/Game/BoardGame/Core/GS_BoardGame.GS_BoardGame_C|GetBoards _asgs_board_game)))))
      (Variables|Default|SetPipe%20Selected%20Number (Math|Integer|%(Integer) (+ (Variables|/Game/BoardGame/Character/BP_BoardCharacter.BP_BoardCharacter_C|GetCurrent%20Board%20Number Pipe%20Using%20Player) 1) (Utilities|Array|Length (Variables|/Game/BoardGame/Core/GS_BoardGame.GS_BoardGame_C|GetBoards _asgs_board_game))))
      (bind _returnvalue (Game|SpawnActorfromClass "/Game/BoardGame/BluePrints/BP_PipeArrow.BP_PipeArrow_C" (Math|Transform|MakeTransform (+ (Transformation|GetActorLocation (Variables|/Game/BoardGame/Core/BP_MainCameraPawn.BP_MainCameraPawn_C|GetTarget%20Actor (Variables|Default|GetMain%20Camera))) "0.000000,0.000000,300.000000") "0, 0, 0" "2.000000,2.000000,2.000000") "Undefined" 0 0))
      (Variables|Default|SetPipe%20Arrow%20Actor _returnvalue)
      (Default|DisableCameraRagging (Variables|Default|GetMain%20Camera)))))

(event Custom|Notify%20Finish%20Move
  ;[1 1 1] PLAYER_MOVE
  (Default|LogicStop (stale Custom|PLAYER_MOVE player))
  (Transformation|SetActorRotation (stale Custom|PLAYER_MOVE player) "0.000000,180.000000,0.000000")
  (Utilities|FlowControl|Delay 1.0)
  (Default|EnableCameraRagging (Variables|Default|GetMain%20Camera))
  (Variables|Default|SetGame%20Step%20String (Utilities|String|Append "PLAYER" (Utilities|String|ToString(Integer) (Variables|/Game/BoardGame/Character/BP_BoardCharacter.BP_BoardCharacter_C|GetPlayerNumber (stale Custom|PLAYER_MOVE player))) "_DOING"))
  (Utilities|FlowControl|DoOnce false) ; enters at Reset
)

(event Custom|Set%20Camera%20Target%20To%20Pipe%20Selected%20Number
  ;[1 1 1] ITEMUSING Pipe Logic
  (bind _asgs_board_game (Utilities|Casting|CastToGS_BoardGame (Game|GetGameState)))
  (Default|SetTargetActor (Variables|Default|GetMain%20Camera) (Utilities|Array|Get(acopy) (Variables|/Game/BoardGame/Core/GS_BoardGame.GS_BoardGame_C|GetBoards _asgs_board_game) (Variables|Default|GetPipe%20Selected%20Number))))

(event Custom|Show%20Player%20In%20Pipe
  (params (Player%20Number :type Integer))
  (bind _players (Variables|Default|GetPlayers))
  (bind _output (Utilities|Array|Get(acopy) _players Player%20Number))
  ;[1 1 1] ITEMUSING Pipe Logic
  (Transformation|SetActorLocation _output (+ (Transformation|GetActorLocation (Variables|Default|GetWarp%20Pipe%20Actor)) "0.000000,0.000000,300.000000") false false)
  (Rendering|SetVisibility (Variables|/Script/Engine.Character|GetMesh _output) true false))

(event Custom|GOTO_MINIGAME
  (bind _main_camera (Variables|Default|GetMain%20Camera))
  ;[1 1 1] GOTO_MINIGAME
  (Variables|Default|SetGame%20Step%20String "PLAYER0_ITEM")
  (Default|DisableCameraRagging _main_camera)
  (Default|SetTargetActor _main_camera))

(event Custom|PLAYER_ITEM
  (params (Player :type BP%20Board%20Character%20Object%20Reference))
  ;[1 1 1] PLAYER_ITEM
  (Utilities|FlowControl|Sequence
    (:then_0
      (Utilities|FlowControl|DoOnce false
        (:Completed
          (Default|SetTargetActor (Variables|Default|GetMain%20Camera) Player)
          (Default|EnableCameraRagging (Variables|Default|GetMain%20Camera))
          (bind _aspc_board_game (Utilities|Casting|CastToPC_BoardGame (Game|GetPlayerController 0)))
          (Default|SelectItemKeyMapping _aspc_board_game (Variables|/Game/BoardGame/Character/BP_BoardCharacter.BP_BoardCharacter_C|GetPlayerNumber Player))
          (bind _asgs_board_game (Utilities|Casting|CastToGS_BoardGame (Game|GetGameState)))
          (Default|ItemUIVisible _asgs_board_game))))
    (:then_1
      (bind _asgs_board_game_2 (Utilities|Casting|CastToGS_BoardGame (Game|GetGameState)))
      (Default|SetItemUI _asgs_board_game_2))))

(event Custom|DEBUG%20PLAYER%20ITEM
  ;[1 1 1] PLAYER_ITEM
  (Development|PrintText (Utilities|Text|FormatText "{num}번째 플레이어 아이템 선택 시작" (Variables|/Game/BoardGame/Character/BP_BoardCharacter.BP_BoardCharacter_C|GetPlayerNumber (stale Custom|PLAYER_ITEM Player)))))

(event Custom|PLAYER_ITEMUSING
  (params (Player :type BP%20Board%20Character%20Object%20Reference))
  ;[1 1 1] PLAYER_ITEMUSING
  (Utilities|FlowControl|Sequence
    (:then_0
      (Utilities|FlowControl|DoOnce false
        (:Completed
          (bind _asps_board_game (Utilities|Casting|CastToPS_BoardGame (Game|GetPlayerState 0)))
          (switch int (Variables|/Game/BoardGame/Core/PS_BoardGame.PS_BoardGame_C|GetItem%20Select%20Number _asps_board_game)
            (:0
              (bind _output_get (Variables|Default|SetUsing%20Item "TO3DICE"))
              (Development|PrintString _output_get)
              (CallFunction|FinishItemUsing :!label _label)
              (Variables|/Game/BoardGame/Core/PS_BoardGame.PS_BoardGame_C|SetItem%20Select%20Number _asps_board_game 0))
            (:1
              (bind _output_get_2 (Variables|Default|SetUsing%20Item "ONLY6DICE"))
              (Development|PrintString _output_get_2)
              (goto _label))
            (:2
              (bind _output_get_3 (Variables|Default|SetUsing%20Item "TO10DICE"))
              (Development|PrintString _output_get_3)
              (goto _label))
            (:3
              (bind _output_get_4 (Variables|Default|SetUsing%20Item "MUSHROOM"))
              (Development|PrintString _output_get_4)
              (goto _label))
            (:4
              (bind _output_get_5 (Variables|Default|SetUsing%20Item "PIPE"))
              (Development|PrintString _output_get_5))))))
    (:then_1
      (switch string (Variables|Default|GetUsing%20Item)
        (:PIPE
          (CallFunction|UsingPipe Player))))))

(event Custom|PLAYER_DICE
  (params (player :type BP%20Board%20Character%20Object%20Reference))
  ;[1 1 1] PLAYER_DICE
  (Utilities|FlowControl|Sequence
    (:then_0
      (Utilities|FlowControl|DoOnce false
        (:Completed
          (Game|SpawnActorfromClass "/Game/BoardGame/BluePrints/BP_DICE.BP_DICE_C" (Math|Transform|MakeTransform (+ (Transformation|GetActorLocation player) "0.000000,0.000000,500.000000") "0, 0, 0" "1.000000,1.000000,1.000000") "Undefined" 0 0))))))

(event Custom|Finish%20Pipe
  (params (Player%20Number :type Integer))
  (bind _players (Variables|Default|GetPlayers))
  (bind _output (Utilities|Array|Get(acopy) _players Player%20Number))
  ;[1 1 1] ITEMUSING Pipe Logic
  (Variables|/Game/BoardGame/Character/BP_BoardCharacter.BP_BoardCharacter_C|SetCurrent%20Board%20Number _output (Variables|Default|GetPipe%20Selected%20Number))
  (Default|SetTargetActor (Variables|Default|GetMain%20Camera) _output)
  (bind _aspc_board_game (Utilities|Casting|CastToPC_BoardGame (Game|GetPlayerController 0)))
  (Default|RollDiceKeyMapping _aspc_board_game Player%20Number)
  (CallFunction|ResetPipeUsing)
  (CallFunction|FinishItemUsing))

(event Custom|Reset%20Pipe%20Using
  ;[1 1 1] ITEMUSING Pipe Logic
  (Utilities|FlowControl|DoOnce false) ; enters at Reset
)

(event Custom|Set%20Player%20Move%20Dice
  ;[1 1 1] Set Player Move Dice
  (bind _asps_board_game (Utilities|Casting|CastToPS_BoardGame (Game|GetPlayerState 0)))
  (switch string (Variables|Default|GetUsing%20Item)
    (:Default
      (Variables|/Game/BoardGame/Core/PS_BoardGame.PS_BoardGame_C|SetPlayer%20Dice%20Count _asps_board_game (Math|Random|RandomIntegerinRange 1 6)))
    (:MUSHROOM
      (Variables|/Game/BoardGame/Core/PS_BoardGame.PS_BoardGame_C|SetPlayer%20Dice%20Count _asps_board_game (Math|Random|RandomIntegerinRange 1 6)))
    (:ONLY6DICE
      (Variables|/Game/BoardGame/Core/PS_BoardGame.PS_BoardGame_C|SetPlayer%20Dice%20Count _asps_board_game 6))
    (:TO10DICE
      (Variables|/Game/BoardGame/Core/PS_BoardGame.PS_BoardGame_C|SetPlayer%20Dice%20Count _asps_board_game (Math|Random|RandomIntegerinRange 1 10)))
    (:TO3DICE
      (Variables|/Game/BoardGame/Core/PS_BoardGame.PS_BoardGame_C|SetPlayer%20Dice%20Count _asps_board_game (Math|Random|RandomIntegerinRange 1 3)))))

(event Custom|For%20Mushroom%20UI
  ;[1 1 1] MUSHROOM UI SETTING
  (bind _asgs_board_game (Utilities|Casting|CastToGS_BoardGame (Game|GetGameState)))
  (Utilities|FlowControl|Sequence
    (:then_0
      (Utilities|FlowControl|DoOnce false
        (:Completed
          (Default|MushroomUIStart (Variables|/Game/BoardGame/Core/GS_BoardGame.GS_BoardGame_C|GetBoardGameUI _asgs_board_game))
          (Utilities|FlowControl|Delay 0.5)
          (Default|MushroomUIMoving (Variables|/Game/BoardGame/Core/GS_BoardGame.GS_BoardGame_C|GetBoardGameUI _asgs_board_game)))))))

(event Custom|Finish%20Mushroom%20UI
  ;[1 1 1] MUSHROOM UI SETTING
  (bind _asps_board_game (Utilities|Casting|CastToPS_BoardGame (Game|GetPlayerState 0)))
  (Variables|/Game/BoardGame/Core/PS_BoardGame.PS_BoardGame_C|SetPlayer%20Dice%20Count _asps_board_game (+ (Variables|/Game/BoardGame/Core/PS_BoardGame.PS_BoardGame_C|GetPlayer%20Dice%20Count _asps_board_game) 3))
  (bind _asgs_board_game (Utilities|Casting|CastToGS_BoardGame (Game|GetGameState)))
  (Default|ShowDiceNumber _asgs_board_game)
  (Utilities|FlowControl|DoOnce false) ; enters at Reset
)

(event Custom|Finish%20Player%20Doing
  ;[1 1 1] PLAYER_DOING
  (Utilities|FlowControl|Sequence
    (:then_0
      (Utilities|FlowControl|DoOnce false) ; enters at Reset
    )
    (:then_1
      (Utilities|FlowControl|DoOnce false) ; enters at Reset
    )
    (:then_3
      (bind _asps_board_game (Utilities|Casting|CastToPS_BoardGame (Game|GetPlayerState 0)))
      (if (<= (Variables|/Game/BoardGame/Core/PS_BoardGame.PS_BoardGame_C|GetPlayer%20Dice%20Count _asps_board_game) 0)
        (if (!= (Variables|/Game/BoardGame/Character/BP_BoardCharacter.BP_BoardCharacter_C|GetPlayerNumber (stale Custom|PLAYER_DOING player)) (- (Utilities|Array|Length (Variables|Default|GetPlayers)) 1))
          (Variables|Default|SetGame%20Step%20String (Utilities|String|Append "PLAYER" (Utilities|String|ToString(Integer) (+ (Variables|/Game/BoardGame/Character/BP_BoardCharacter.BP_BoardCharacter_C|GetPlayerNumber (stale Custom|PLAYER_DOING player)) 1)) "_ITEM"))
          (else
            (Variables|Default|SetGame%20Step%20String "GOTO_MINIGAME")))
        (else
          (Variables|Default|SetGame%20Step%20String (Utilities|String|Append "PLAYER" (Utilities|String|ToString(Integer) (Variables|/Game/BoardGame/Character/BP_BoardCharacter.BP_BoardCharacter_C|GetPlayerNumber (stale Custom|PLAYER_DOING player))) "_MOVE")))))))

(event Custom|Check%20Current%20Is%20Special%20Board
  (params (Player :type BP%20Board%20Character%20Object%20Reference))
  (Utilities|FlowControl|DoOnce false
    (:Completed
      (bind _asgs_board_game (Utilities|Casting|CastToGS_BoardGame (Game|GetGameState)))
      (Class|BIFDoingBoards|DoingSpecialBoard(Message) (Utilities|Array|Get(acopy) (Variables|/Game/BoardGame/Core/GS_BoardGame.GS_BoardGame_C|GetBoards _asgs_board_game) (Variables|/Game/BoardGame/Character/BP_BoardCharacter.BP_BoardCharacter_C|GetCurrent%20Board%20Number Player)) (Variables|/Game/BoardGame/Character/BP_BoardCharacter.BP_BoardCharacter_C|GetPlayerNumber Player)))))

(event Custom|Set%20Player%20UI%20At%20Begin%20Play
  ;[1 1 1] BeginPlay
  (for _array_element (Variables|Default|GetPlayers)
    (Default|SetPlayerUI _array_element)))

(event Custom|Send%20Player%20Text%20Ok%20Or%20No
  (params (Player%20Number :type Integer) (Ok? :type Boolean))
  (bind _players (Variables|Default|GetPlayers))
  (bind _output (Utilities|Array|Get(acopy) _players Player%20Number))
  (bind _asgs_board_game (Utilities|Casting|CastToGS_BoardGame (Game|GetGameState)))
  (bind _asbp_star_board (Utilities|Casting|CastToBP_StarBoard (Utilities|Array|Get(acopy) (Variables|/Game/BoardGame/Core/GS_BoardGame.GS_BoardGame_C|GetBoards _asgs_board_game) (Variables|/Game/BoardGame/Character/BP_BoardCharacter.BP_BoardCharacter_C|GetCurrent%20Board%20Number (Utilities|Array|Get(acopy) (Variables|Default|GetPlayers) Player%20Number)))))
  (if Ok?
    (Default|BuyStar (Variables|/Game/BoardGame/Core/GS_BoardGame.GS_BoardGame_C|GetBoardGameUI _asgs_board_game))
    (Default|AddPlayerCoin _output -20)
    (Default|AddPlayerStar _output 1)
    (Default|RemoveStarHere _asbp_star_board)
    (CallFunction|CreateNewStar _asbp_star_board Player%20Number)
    (else
      (CallFunction|FinishTextDoing))))

(event Custom|Finish%20Text%20Doing
  (bind _asgs_board_game (Utilities|Casting|CastToGS_BoardGame (Game|GetGameState)))
  (Default|HiddenTextUI (Variables|/Game/BoardGame/Core/GS_BoardGame.GS_BoardGame_C|GetBoardGameUI _asgs_board_game))
  (bind _aspc_board_game (Utilities|Casting|CastToPC_BoardGame (Game|GetPlayerController 0)))
  (Default|RemoveAllKeyMapping _aspc_board_game)
  (CallFunction|FinishPlayerDoing))

(event Custom|Create%20New%20Star
  (params (Now%20Star :type BP%20Star%20Board%20Object%20Reference) (Now%20Player%20Number :type Integer))
  (bind _star_boards (Variables|Default|GetStar%20Boards))
  (bind _main_camera (Variables|Default|GetMain%20Camera))
  (bind _main_camera_2 (Variables|Default|GetMain%20Camera))
  (bind _outitem (Utilities|Array|Random _star_boards))
  (Variables|Default|SetNew%20Star%20Target _outitem)
  (if (== (Variables|/Game/BoardGame/BluePrints/BP_Board.BP_Board_C|GetBoard%20Order Now%20Star) (Variables|/Game/BoardGame/BluePrints/BP_Board.BP_Board_C|GetBoard%20Order _outitem))
    (CallFunction|CreateNewStar Now%20Star Now%20Player%20Number)
    (else
      (bind _asgs_board_game (Utilities|Casting|CastToGS_BoardGame (Game|GetGameState)))
      (Default|NewStarText (Variables|/Game/BoardGame/Core/GS_BoardGame.GS_BoardGame_C|GetBoardGameUI _asgs_board_game))
      (Default|SetStarHere (Variables|Default|GetNew%20Star%20Target))
      (Default|SetTargetActor _main_camera_2 (Variables|Default|GetNew%20Star%20Target))
      (Default|EnableCameraRagging _main_camera_2)
      (Utilities|FlowControl|Delay 2.0)
      (Default|DisableCameraRagging _main_camera)
      (Default|SetTargetActor _main_camera (Utilities|Array|Get(acopy) (Variables|Default|GetPlayers) Now%20Player%20Number))
      (CallFunction|FinishTextDoing))))

(event Custom|Pipe%20Select%20Board
  (params (Player%20Number :type Integer))
  (bind _players (Variables|Default|GetPlayers))
  (bind _output (Utilities|Array|Get(acopy) _players Player%20Number))
  (bind _returnvalue (Transformation|GetActorLocation _output))
  ;[1 1 1] ITEMUSING Pipe Logic
  (if (== (Variables|/Game/BoardGame/Character/BP_BoardCharacter.BP_BoardCharacter_C|GetCurrent%20Board%20Number _output) (Variables|Default|GetPipe%20Selected%20Number))
    (Development|PrintText "현재 위치한 보드라서 사용할 수 없습니다!!")
    (else
      (bind _aspc_board_game (Utilities|Casting|CastToPC_BoardGame (Game|GetPlayerController 0)))
      (Default|RemoveAllKeyMapping _aspc_board_game)
      (Default|SetTargetActor (Variables|Default|GetMain%20Camera) _output)
      (Actor|DestroyActor (Variables|Default|GetPipe%20Arrow%20Actor))
      (bind _returnvalue_2 (Game|SpawnActorfromClass "/Game/BoardGame/BluePrints/BP_WarpPipe.BP_WarpPipe_C" (Math|Transform|MakeTransform (Math|Vector|MakeVector (.x _returnvalue) (.y _returnvalue) -434.0) "0, 0, 0" "1.000000,1.000000,1.000000") "Undefined" 0 0))
      (bind _output_get (Variables|Default|SetWarp%20Pipe%20Actor _returnvalue_2))
      (Variables|/Game/BoardGame/BluePrints/BP_WarpPipe.BP_WarpPipe_C|Setwho%20Player? _output_get (Variables|/Game/BoardGame/Character/BP_BoardCharacter.BP_BoardCharacter_C|GetPlayerNumber _output)))))

(event Custom|Finish%20Item%20Using
  ;[1 1 1] PLAYER_ITEMUSING
  (Variables|Default|SetGame%20Step%20String (Utilities|String|Append "PLAYER" (Utilities|String|ToString(Integer) (Variables|/Game/BoardGame/Character/BP_BoardCharacter.BP_BoardCharacter_C|GetPlayerNumber (stale Custom|PLAYER_ITEMUSING Player))) "_DICE"))
  (Utilities|FlowControl|DoOnce false) ; enters at Reset
)

(event Custom|PLAYER_MOVE
  (params (player :type BP%20Board%20Character%20Object%20Reference))
  ;[1 1 1] PLAYER_MOVE
  (Utilities|FlowControl|Sequence
    (:then_0
      (Utilities|FlowControl|DoOnce false
        (:Completed
          (Default|DisableCameraRagging (Variables|Default|GetMain%20Camera))
          (Default|LogicRestart player))))
    (:then_1
      (bind _asgs_board_game (Utilities|Casting|CastToGS_BoardGame (Game|GetGameState)))
      (Default|ShowDiceNumber _asgs_board_game))))

(event Custom|PLAYER_DOING
  (params (player :type BP%20Board%20Character%20Object%20Reference))
  ;[1 1 1] PLAYER_DOING
  (Utilities|FlowControl|Sequence
    (:then_0
      (Utilities|FlowControl|DoOnce false
        (:Completed
          (bind _asgs_board_game (Utilities|Casting|CastToGS_BoardGame (Game|GetGameState)))
          (Default|HiddenDiceNumber _asgs_board_game)
          (CallFunction|CheckCurrentIsSpecialBoard player))))))

(event Custom|Pipe%20Move%20Board
  (params (Move%20Input%20Value :type Integer))
  ;[1 1 1] ITEMUSING Pipe Logic
  (bind _asgs_board_game (Utilities|Casting|CastToGS_BoardGame (Game|GetGameState)))
  (bind _output_get (Variables|Default|SetPipe%20Selected%20Number (Math|Integer|%(Integer) (+ (Variables|Default|GetPipe%20Selected%20Number) Move%20Input%20Value (Utilities|Array|Length (Variables|/Game/BoardGame/Core/GS_BoardGame.GS_BoardGame_C|GetBoards _asgs_board_game))) (Utilities|Array|Length (Variables|/Game/BoardGame/Core/GS_BoardGame.GS_BoardGame_C|GetBoards _asgs_board_game)))))
  (Transformation|SetActorLocation (Variables|Default|GetPipe%20Arrow%20Actor) (+ (Transformation|GetActorLocation (Utilities|Array|Get(acopy) (Variables|/Game/BoardGame/Core/GS_BoardGame.GS_BoardGame_C|GetBoards _asgs_board_game) _output_get)) "0.000000,0.000000,300.000000") false false)
  (Default|SetTargetActor (Variables|Default|GetMain%20Camera) (Utilities|Array|Get(acopy) (Variables|/Game/BoardGame/Core/GS_BoardGame.GS_BoardGame_C|GetBoards _asgs_board_game) _output_get)))

(event Custom|Player%20Roll%20Dice
  ;[1 1 1] PLAYER_DICE
  (CallFunction|SetPlayerMoveDice)
  (bind _aspc_board_game (Utilities|Casting|CastToPC_BoardGame (Game|GetPlayerController 0)))
  (Default|RemoveAllKeyMapping _aspc_board_game)
  (bind _asgs_board_game (Utilities|Casting|CastToGS_BoardGame (Game|GetGameState)))
  (Default|ShowDiceNumber _asgs_board_game)
  (if (Utilities|Enum|Equal(Enum) (Variables|Default|GetUsing%20Item) "MUSHROOM")
    (CallFunction|ForMushroomUI)
    (Utilities|FlowControl|Delay 2.0)
    (else
      (Utilities|FlowControl|Delay 1.0)))
  (Development|PrintText "2")
  (Variables|Default|SetGame%20Step%20String (Utilities|String|Append "PLAYER" (Utilities|String|ToString(Integer) (Variables|/Game/BoardGame/Character/BP_BoardCharacter.BP_BoardCharacter_C|GetPlayerNumber (stale Custom|PLAYER_DICE player))) "_MOVE"))
  (Utilities|FlowControl|DoOnce false) ; enters at Reset
)

(event Custom|Pipe%20Warp
  (params (Player%20Number :type Integer))
  ;[1 1 1] ITEMUSING Pipe Logic
  (Rendering|SetVisibility (Variables|/Script/Engine.Character|GetMesh (Utilities|Array|Get(acopy) (Variables|Default|GetPlayers) Player%20Number)) false false)
  (bind _asgs_board_game (Utilities|Casting|CastToGS_BoardGame (Game|GetGameState)))
  (Transformation|SetActorLocation (Variables|Default|GetWarp%20Pipe%20Actor) (Math|Vector|MakeVector (.x (Transformation|GetActorLocation (Utilities|Array|Get(acopy) (Variables|/Game/BoardGame/Core/GS_BoardGame.GS_BoardGame_C|GetBoards _asgs_board_game) (Variables|Default|GetPipe%20Selected%20Number)))) (.y (Transformation|GetActorLocation (Utilities|Array|Get(acopy) (Variables|/Game/BoardGame/Core/GS_BoardGame.GS_BoardGame_C|GetBoards _asgs_board_game) (Variables|Default|GetPipe%20Selected%20Number)))) -434.0) false false))

(event EventBeginPlay
  ;[1 1 1] BeginPlay
  (bind _returnvalue (Actor|GetActorOfClass "/Game/BoardGame/Core/BP_MainCameraPawn.BP_MainCameraPawn_C"))
  (Variables|Default|SetMain%20Camera _returnvalue)
  (bind _outactors (Actor|GetAllActorsOfClass "/Game/BoardGame/Character/BP_BoardCharacter.BP_BoardCharacter_C"))
  (CallFunction|GetPlayerArray _outactors)
  (bind _outactors_2 (Actor|GetAllActorsOfClass "/Game/BoardGame/BluePrints/BP_StarBoard.BP_StarBoard_C"))
  (bind _output_get (Variables|Default|SetStar%20Boards _outactors_2))
  (Default|SetStarHere (Utilities|Array|Get(acopy) _output_get))
  (Variables|Default|SetGame%20Step%20String "PLAYER0_ITEM"))

(event EventTick
  (params (DeltaSeconds :type Float%20%28single-precision%29))
  (bind _players (Variables|Default|GetPlayers))
  (bind _players_2 (Variables|Default|GetPlayers))
  (bind _output (Utilities|Array|Get(acopy) _players 1))
  (bind _output_2 (Utilities|Array|Get(acopy) _players_2))
  ;[1 1 1] Event Tick Logic
  (switch string (Variables|Default|GetGame%20Step%20String)
    (:PLAYER0_ITEM
      (CallFunction|PLAYERITEM _output_2))
    (:PLAYER0_ITEMUSING
      (CallFunction|PLAYERITEMUSING _output_2))
    (:PLAYER0_DICE
      (CallFunction|PLAYERDICE _output_2))
    (:PLAYER0_MOVE
      (CallFunction|PLAYERMOVE _output_2))
    (:PLAYER0_DOING
      (CallFunction|PLAYERDOING _output_2))
    (:PLAYER1_ITEM
      (CallFunction|PLAYERITEM _output))
    (:PLAYER1_ITEMUSING
      (CallFunction|PLAYERITEMUSING _output))
    (:PLAYER1_DICE
      (CallFunction|PLAYERDICE _output))
    (:PLAYER1_MOVE
      (CallFunction|PLAYERMOVE _output))
    (:PLAYER1_DOING
      (CallFunction|PLAYERDOING _output))
    (:GOTO_MINIGAME
      (CallFunction|GOTOMINIGAME))))

(fn ConstructionScript)

(fn GetPlayerArray
  (params (GetAllActorsOfCharacter :type Array%20of%20BP%20Board%20Character%20Object%20References))
  (for _array_element GetAllActorsOfCharacter :!label _label
    (if (== (Variables|/Game/BoardGame/Character/BP_BoardCharacter.BP_BoardCharacter_C|GetPlayerNumber _array_element) (Utilities|Array|Length (Variables|Default|GetPlayers)))
      (Utilities|Array|Add (Variables|Default|GetPlayers) _array_element)
      (goto _label))))