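; BP_MainCameraPawn is the board game's main camera pawn, switching between a fixed main view and follow views of two players.
; Target starts as the main camera, and every Tick it selects either a fixed location or a position at a constant offset from Player1 or Player2.
; DoOnce gates that reset one another set the pitch on view changes, shallower for players and steeper for the main view.
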(event EventBeginPlay
  (Variables|Default|SetTarget "MAINCAMERA"))

(event Collision|EventActorBeginOverlap
  (params (OtherActor :type Actor%20Object%20Reference)))

(event EventTick
  (params (DeltaSeconds :type Float%20%28single-precision%29))
  (switch string (Variables|Default|GetTarget)
    (:PLAYER1
      (Transformation|SetActorLocation (+ (Transformation|GetActorLocation (Variables|Default|GetPlayer1)) "-2500.000000,0.000000,1500.000000") false false)
      (Utilities|FlowControl|DoOnce false :!label _label
        (:Completed
          (Transformation|SetActorRotation "-30.000000,0.000000,0.000000")
          (goto _label_3 Reset))))
    (:PLAYER2
      (Transformation|SetActorLocation (+ (Transformation|GetActorLocation (Variables|Default|GetPlayer2)) "-2500.000000,0.000000,1500.000000") false false)
      (Utilities|FlowControl|DoOnce false :!label _label_2
        (:Completed
          (Transformation|SetActorRotation "-30.000000,0.000000,0.000000")
          (goto _label_3 Reset))))
    (:MAINCAMERA
      (Transformation|SetActorLocation "-15979.000000,-649.000000,3654.000000" false false)
      (Utilities|FlowControl|DoOnce false :!label _label_3
        (:Completed
          (Transformation|SetActorRotation "-45.000000,0.000000,0.000000")
          (Utilities|FlowControl|Sequence
            (:then_0
              (goto _label Reset))
            (:then_1
              (goto _label_2 Reset))))))))

(fn ConstructionScript)