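; Board game player controller that handles input for two players through turn phases: item selection, dice roll and Pipe item targeting.
; Each phase clears all mapping contexts, then adds that player's Enhanced Input context.
; Item changes update ItemSelectNumber on player state 0 for both players; confirming calls GM_BoardGame, then UsingDice picks roll or Pipe controls.
; Rolling makes the player jump behind resettable DoOnce gates, while Pipe input forwards to GM_BoardGame.
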(event Custom|ChangeItem
  (params (Action%20Value :type Integer))
  ;[1 1 1] Select Item 0P, 1P
  (bind _asps_board_game (Utilities|Casting|CastToPS_BoardGame (Game|GetPlayerState 0)))
  (Variables|/Game/BoardGame/Core/PS_BoardGame.PS_BoardGame_C|SetItem%20Select%20Number _asps_board_game (Math|Integer|Clamp(Integer) (+ (Variables|/Game/BoardGame/Core/PS_BoardGame.PS_BoardGame_C|GetItem%20Select%20Number _asps_board_game) Action%20Value) 0 4)))

(event Custom|Select%20Item%20Key%20Mapping
  (params (Player%20Number :type Integer))
  (bind _returnvalue (PlayerController|LocalPlayerSubsystems|GetEnhancedInputLocalPlayerSubsystem))
  ;[1 1 1] Select Item Key Mapping
  (CallFunction|RemoveAllKeyMapping)
  (switch int Player%20Number
    (:0
      (Input|AddMappingContext _returnvalue "/Game/BoardGame/Core/Input/SelectItem/IMC_1PSelectItem.IMC_1PSelectItem" 0 "(bIgnoreAllPressedKeysUntilRelease=True,bForceImmediately=False)"))
    (:1
      (Input|AddMappingContext _returnvalue "/Game/BoardGame/Core/Input/SelectItem/IMC_2PSelectItem.IMC_2PSelectItem" 0 "(bIgnoreAllPressedKeysUntilRelease=True,bForceImmediately=False)"))))

(event Custom|Roll%20Dice%20Key%20Mapping
  (params (Player%20Number :type Integer))
  (bind _returnvalue (PlayerController|LocalPlayerSubsystems|GetEnhancedInputLocalPlayerSubsystem))
  ;[1 1 1] Roll Dice Key Mapping
  (CallFunction|RemoveAllKeyMapping)
  (switch int Player%20Number
    (:0
      (Input|AddMappingContext _returnvalue "/Game/BoardGame/Core/Input/RollDice/IMC_1PRollDice.IMC_1PRollDice" 0 "(bIgnoreAllPressedKeysUntilRelease=True,bForceImmediately=False)"))
    (:1
      (Input|AddMappingContext _returnvalue "/Game/BoardGame/Core/Input/RollDice/IMC_2PRollDice.IMC_2PRollDice" 0 "(bIgnoreAllPressedKeysUntilRelease=True,bForceImmediately=False)"))))

(event Custom|Reset%20Do%20Once%20for%20Player2%20Roll%20Dice
  ;[1 1 1] Roll Dice_1P, 2P
  (Utilities|FlowControl|DoOnce false) ; enters at Reset
)

(event Custom|Remove%20All%20Key%20Mapping
  (bind _returnvalue (PlayerController|LocalPlayerSubsystems|GetEnhancedInputLocalPlayerSubsystem))
  ;[1 1 1] Remove Key Mapping
  (Input|RemoveMappingContext _returnvalue "/Game/BoardGame/Core/Input/RollDice/IMC_1PRollDice.IMC_1PRollDice" "(bIgnoreAllPressedKeysUntilRelease=True,bForceImmediately=False)")
  (Input|RemoveMappingContext _returnvalue "/Game/BoardGame/Core/Input/RollDice/IMC_2PRollDice.IMC_2PRollDice" "(bIgnoreAllPressedKeysUntilRelease=True,bForceImmediately=False)")
  (Input|RemoveMappingContext _returnvalue "/Game/BoardGame/Core/Input/SelectItem/IMC_1PSelectItem.IMC_1PSelectItem" "(bIgnoreAllPressedKeysUntilRelease=True,bForceImmediately=False)")
  (Input|RemoveMappingContext _returnvalue "/Game/BoardGame/Core/Input/SelectItem/IMC_2PSelectItem.IMC_2PSelectItem" "(bIgnoreAllPressedKeysUntilRelease=True,bForceImmediately=False)")
  (Input|RemoveMappingContext _returnvalue "/Game/BoardGame/Core/Input/ItemUsing/IMC_0PPipe1.IMC_0PPipe1" "(bIgnoreAllPressedKeysUntilRelease=True,bForceImmediately=False)")
  (Input|RemoveMappingContext _returnvalue "/Game/BoardGame/Core/Input/ItemUsing/IMC_1PPipe.IMC_1PPipe" "(bIgnoreAllPressedKeysUntilRelease=True,bForceImmediately=False)"))

(event Custom|Reset%20Do%20Once%20For%20Player1%20Roll%20Dice
  ;[1 1 1] Roll Dice_1P, 2P
  (Utilities|FlowControl|DoOnce false) ; enters at Reset
)

(event Custom|ItemUsing%20Pipe%20Key%20Mapping
  (params (Player%20Number :type Integer))
  (bind _returnvalue (PlayerController|LocalPlayerSubsystems|GetEnhancedInputLocalPlayerSubsystem))
  ;[1 1 1] ItemUsing Pipe Key Mapping (0P, 1P)
  (CallFunction|RemoveAllKeyMapping)
  (switch int Player%20Number
    (:0
      (Input|AddMappingContext _returnvalue "/Game/BoardGame/Core/Input/ItemUsing/IMC_0PPipe1.IMC_0PPipe1" 0 "(bIgnoreAllPressedKeysUntilRelease=True,bForceImmediately=False)"))
    (:1
      (Input|AddMappingContext _returnvalue "/Game/BoardGame/Core/Input/ItemUsing/IMC_1PPipe.IMC_1PPipe" 0 "(bIgnoreAllPressedKeysUntilRelease=True,bForceImmediately=False)"))))

(event Custom|Notify%20Reset%20For%20Roll%20Dice
  (params (PlayerNumber :type Integer))
  ;[1 1 1] Roll Dice_1P, 2P
  (switch int PlayerNumber
    (:0
      (CallFunction|ResetDoOnceforPlayer1RollDice))
    (:1
      (CallFunction|ResetDoOnceforPlayer2RollDice))))

(event Input|EnhancedActionEvents|EnhancedInputActionIA_2PChangeItem
  (params (ActionValue :type Float%20%28double-precision%29) (ElapsedSeconds :type Float%20%28double-precision%29) (TriggeredSeconds :type Float%20%28double-precision%29) (InputAction :type Input%20Action%20Object%20Reference :default "/Game/BoardGame/Core/Input/SelectItem/IA_2PChangeItem.IA_2PChangeItem"))
  ;[1 1 1] Select Item 0P, 1P
  (:Started
    (CallFunction|ChangeItem (Math|Float|Truncate ActionValue))))

(event Input|EnhancedActionEvents|EnhancedInputActionIA_1PSelectItem
  (params (ActionValue :type Boolean) (ElapsedSeconds :type Float%20%28double-precision%29) (TriggeredSeconds :type Float%20%28double-precision%29) (InputAction :type Input%20Action%20Object%20Reference :default "/Game/BoardGame/Core/Input/SelectItem/IA_1PSelectItem.IA_1PSelectItem"))
  (bind _returnvalue (Game|GetGameMode))
  ;[1 1 1] Select Item 0P, 1P
  (:Started
    (bind _asgm_board_game (Utilities|Casting|CastToGM_BoardGame _returnvalue))
    (Default|FinishItemSelect _asgm_board_game))
  (:Completed
    (bind _asgm_board_game_2 (Utilities|Casting|CastToGM_BoardGame _returnvalue))
    (switch string (Variables|/Game/BoardGame/Core/GM_BoardGame.GM_BoardGame_C|GetUsing%20Dice _asgm_board_game_2)
      (:Default
        (CallFunction|RollDiceKeyMapping))
      (:PIPE
        (CallFunction|ItemUsingPipeKeyMapping)))))

(event Input|EnhancedActionEvents|EnhancedInputActionIA_0P_PIPE_MoveBoard
  (params (ActionValue :type Float%20%28double-precision%29) (ElapsedSeconds :type Float%20%28double-precision%29) (TriggeredSeconds :type Float%20%28double-precision%29) (InputAction :type Input%20Action%20Object%20Reference :default "/Game/BoardGame/Core/Input/ItemUsing/IA_0P_PIPE_MoveBoard.IA_0P_PIPE_MoveBoard"))
  (:Started
    (bind _asgm_board_game (Utilities|Casting|CastToGM_BoardGame (Game|GetGameMode)))
    (Default|PipeMoveBoard _asgm_board_game (Math|Float|Truncate ActionValue))))

(event Input|EnhancedActionEvents|EnhancedInputActionIA_1PChangeItem
  (params (ActionValue :type Float%20%28double-precision%29) (ElapsedSeconds :type Float%20%28double-precision%29) (TriggeredSeconds :type Float%20%28double-precision%29) (InputAction :type Input%20Action%20Object%20Reference :default "/Game/BoardGame/Core/Input/SelectItem/IA_1PChangeItem.IA_1PChangeItem"))
  ;[1 1 1] Select Item 0P, 1P
  (:Started
    (CallFunction|ChangeItem (Math|Float|Truncate ActionValue))))

(event Input|EnhancedActionEvents|EnhancedInputActionIA_1PRollDice
  (params (ActionValue :type Boolean) (ElapsedSeconds :type Float%20%28double-precision%29) (TriggeredSeconds :type Float%20%28double-precision%29) (InputAction :type Input%20Action%20Object%20Reference :default "/Game/BoardGame/Core/Input/RollDice/IA_1PRollDice.IA_1PRollDice"))
  ;[1 1 1] Roll Dice_1P, 2P
  (:Started
    (Utilities|FlowControl|DoOnce false
      (:Completed
        (bind _asgm_board_game (Utilities|Casting|CastToGM_BoardGame (Game|GetGameMode)))
        (Character|Jump (Utilities|Array|Get(acopy) (Variables|/Game/BoardGame/Core/GM_BoardGame.GM_BoardGame_C|GetPlayers _asgm_board_game)))))))

(event Input|EnhancedActionEvents|EnhancedInputActionIA_2PRollDice
  (params (ActionValue :type Boolean) (ElapsedSeconds :type Float%20%28double-precision%29) (TriggeredSeconds :type Float%20%28double-precision%29) (InputAction :type Input%20Action%20Object%20Reference :default "/Game/BoardGame/Core/Input/RollDice/IA_2PRollDice.IA_2PRollDice"))
  ;[1 1 1] Roll Dice_1P, 2P
  (:Started
    (Utilities|FlowControl|DoOnce false
      (:Completed
        (bind _asgm_board_game (Utilities|Casting|CastToGM_BoardGame (Game|GetGameMode)))
        (Character|Jump (Utilities|Array|Get(acopy) (Variables|/Game/BoardGame/Core/GM_BoardGame.GM_BoardGame_C|GetPlayers _asgm_board_game) 1))))))

(event Input|EnhancedActionEvents|EnhancedInputActionIA_0P_PIPE_SelectBoard
  (params (ActionValue :type Boolean) (ElapsedSeconds :type Float%20%28double-precision%29) (TriggeredSeconds :type Float%20%28double-precision%29) (InputAction :type Input%20Action%20Object%20Reference :default "/Game/BoardGame/Core/Input/ItemUsing/IA_0P_PIPE_SelectBoard.IA_0P_PIPE_SelectBoard"))
  (:Started
    (bind _asgm_board_game (Utilities|Casting|CastToGM_BoardGame (Game|GetGameMode)))
    (Default|PipeSelectBoard _asgm_board_game)))

(event Input|EnhancedActionEvents|EnhancedInputActionIA_2PSelectItem
  (params (ActionValue :type Boolean) (ElapsedSeconds :type Float%20%28double-precision%29) (TriggeredSeconds :type Float%20%28double-precision%29) (InputAction :type Input%20Action%20Object%20Reference :default "/Game/BoardGame/Core/Input/SelectItem/IA_2PSelectItem.IA_2PSelectItem"))
  (bind _returnvalue (Game|GetGameMode))
  ;[1 1 1] Select Item 0P, 1P
  (:Started
    (bind _asgm_board_game (Utilities|Casting|CastToGM_BoardGame _returnvalue))
    (Default|FinishItemSelect _asgm_board_game))
  (:Completed
    (bind _asgm_board_game_2 (Utilities|Casting|CastToGM_BoardGame _returnvalue))
    (switch string (Variables|/Game/BoardGame/Core/GM_BoardGame.GM_BoardGame_C|GetUsing%20Dice _asgm_board_game_2)
      (:Default
        (CallFunction|RollDiceKeyMapping 1))
      (:PIPE
        (CallFunction|ItemUsingPipeKeyMapping 1)))))

(event Input|EnhancedActionEvents|EnhancedInputActionIA_1P_PIPE_MoveBoard
  (params (ActionValue :type Float%20%28double-precision%29) (ElapsedSeconds :type Float%20%28double-precision%29) (TriggeredSeconds :type Float%20%28double-precision%29) (InputAction :type Input%20Action%20Object%20Reference :default "/Game/BoardGame/Core/Input/ItemUsing/IA_1P_PIPE_MoveBoard.IA_1P_PIPE_MoveBoard"))
  (:Started
    (bind _asgm_board_game (Utilities|Casting|CastToGM_BoardGame (Game|GetGameMode)))
    (Default|PipeMoveBoard _asgm_board_game (Math|Float|Truncate ActionValue))))

(event Input|EnhancedActionEvents|EnhancedInputActionIA_1P_PIPE_SelectBoard
  (params (ActionValue :type Boolean) (ElapsedSeconds :type Float%20%28double-precision%29) (TriggeredSeconds :type Float%20%28double-precision%29) (InputAction :type Input%20Action%20Object%20Reference :default "/Game/BoardGame/Core/Input/ItemUsing/IA_1P_PIPE_SelectBoard.IA_1P_PIPE_SelectBoard"))
  (:Started
    (bind _asgm_board_game (Utilities|Casting|CastToGM_BoardGame (Game|GetGameMode)))
    (Default|PipeSelectBoard _asgm_board_game 1)))

(fn ConstructionScript)