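; Gas station special board square for the board game that blows up the player landing on it and costs them 10 coins.
; DoingSpecialBoard spawns an explosion at the station and launches the player's mesh with a physics impulse along the station-to-square direction cached at BeginPlay.
; After a delay it turns physics off, restores the mesh's saved relative transform, then tells GM_BoardGame the player's action is finished.
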(event EventBeginPlay
  (|CallParentFunction)
  (Variables|Default|SetExploding%20Direction (- (Transformation|GetActorLocation) (Variables|Default|GetGas%20Station%20Location))))

(event Collision|EventActorBeginOverlap
  (params (OtherActor :type Actor%20Object%20Reference))
  (|CallParentFunction OtherActor) ; This node is disabled and will not be called.\nDrag off pins to build functionality.
)

(event EventTick
  (params (DeltaSeconds :type Float%20%28single-precision%29))
  (|CallParentFunction DeltaSeconds) ; This node is disabled and will not be called.\nDrag off pins to build functionality.
)

(event EventDoingSpecialBoard
  (params (Player%20Number :type Integer))
  (bind _asgm_board_game (Utilities|Casting|CastToGM_BoardGame (Game|GetGameMode)))
  (Effects|SpawnEmitteratLocation "/Game/StarterContent/Particles/P_Explosion.P_Explosion" (Variables|Default|GetGas%20Station%20Location) "0, 0, 0" "15.000000,15.000000,15.000000")
  (Collision|SetCollisionEnabled (Variables|/Script/Engine.Character|GetMesh (Utilities|Array|Get(acopy) (Variables|/Game/BoardGame/Core/GM_BoardGame.GM_BoardGame_C|GetPlayers _asgm_board_game) Player%20Number)) "PhysicsOnly")
  (Physics|SetSimulatePhysics (Variables|/Script/Engine.Character|GetMesh (Utilities|Array|Get(acopy) (Variables|/Game/BoardGame/Core/GM_BoardGame.GM_BoardGame_C|GetPlayers _asgm_board_game) Player%20Number)) true)
  (Variables|Default|SetLast%20Relative%20Location (Variables|/Script/Engine.SceneComponent|GetRelativeLocation (Variables|/Script/Engine.Character|GetMesh (Utilities|Array|Get(acopy) (Variables|/Game/BoardGame/Core/GM_BoardGame.GM_BoardGame_C|GetPlayers _asgm_board_game) Player%20Number))))
  (Variables|Default|SetLast%20Relative%20Rotation (Variables|/Script/Engine.SceneComponent|GetRelativeRotation (Variables|/Script/Engine.Character|GetMesh (Utilities|Array|Get(acopy) (Variables|/Game/BoardGame/Core/GM_BoardGame.GM_BoardGame_C|GetPlayers _asgm_board_game) Player%20Number))))
  (Physics|AddImpulse (Variables|/Script/Engine.Character|GetMesh (Utilities|Array|Get(acopy) (Variables|/Game/BoardGame/Core/GM_BoardGame.GM_BoardGame_C|GetPlayers _asgm_board_game) Player%20Number)) (* (Variables|Default|GetExploding%20Direction) 7e+03) "None" false)
  (Default|AddPlayerCoin (Utilities|Array|Get(acopy) (Variables|/Game/BoardGame/Core/GM_BoardGame.GM_BoardGame_C|GetPlayers _asgm_board_game) Player%20Number) -10)
  (Utilities|FlowControl|Delay 3.0)
  (Physics|SetSimulatePhysics (Variables|/Script/Engine.Character|GetMesh (Utilities|Array|Get(acopy) (Variables|/Game/BoardGame/Core/GM_BoardGame.GM_BoardGame_C|GetPlayers _asgm_board_game) Player%20Number)) false)
  (Collision|SetCollisionEnabled (Variables|/Script/Engine.Character|GetMesh (Utilities|Array|Get(acopy) (Variables|/Game/BoardGame/Core/GM_BoardGame.GM_BoardGame_C|GetPlayers _asgm_board_game) Player%20Number)) "NoCollision")
  (Transformation|SetRelativeLocationAndRotation (Variables|/Script/Engine.Character|GetMesh (Utilities|Array|Get(acopy) (Variables|/Game/BoardGame/Core/GM_BoardGame.GM_BoardGame_C|GetPlayers _asgm_board_game) Player%20Number)) (Variables|Default|GetLast%20Relative%20Location) (Variables|Default|GetLast%20Relative%20Rotation) false false)
  (Utilities|FlowControl|Delay 1.5)
  (Default|FinishPlayerDoing _asgm_board_game))

(fn ConstructionScript
  (|CallParentFunction))