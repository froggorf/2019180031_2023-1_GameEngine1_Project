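; BP_MinusBoard is a penalty board space for the board game that takes coins from the player it acts on.
; Its DoingSpecialBoard event casts the game mode to GM_BoardGame and subtracts three coins from the indexed player through AddPlayerCoin.
; It then calls FinishPlayerDoing on the game mode to end that player's action.
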(event EventBeginPlay
  (|CallParentFunction) ; This node is disabled and will not be called.\nDrag off pins to build functionality.
)

(event Collision|EventActorBeginOverlap
  (params (OtherActor :type Actor%20Object%20Reference))
  (|CallParentFunction OtherActor) ; This node is disabled and will not be called.\nDrag off pins to build functionality.
)

(event EventTick
  (params (DeltaSeconds :type Float%20%28single-precision%29))
  (|CallParentFunction DeltaSeconds) ; This node is disabled and will not be called.\nDrag off pins to build functionality.
)

(event EventDoingSpecialBoard
  (params (Player%20Number :type Integer))
  (bind _asgm_board_game (Utilities|Casting|CastToGM_BoardGame (Game|GetGameMode)))
  (Default|AddPlayerCoin (Utilities|Array|Get(acopy) (Variables|/Game/BoardGame/Core/GM_BoardGame.GM_BoardGame_C|GetPlayers _asgm_board_game) Player%20Number) -3)
  (Default|FinishPlayerDoing _asgm_board_game))

(fn ConstructionScript
  (|CallParentFunction))