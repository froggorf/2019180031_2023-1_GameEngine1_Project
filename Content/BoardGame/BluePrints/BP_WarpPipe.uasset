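; Board-game warp pipe actor that animates a player being swallowed, warped and released.
; Tick runs a flag-chained sequence: pipe rises, Cube component lowers, pipe rises again, Cube lifts, then pipe sinks and destroys itself.
; Between phases it calls GM_BoardGame to retarget the camera, warp and show WhoPlayer, then finish the turn's pipe event.
; Movement is constant-speed, delta-time stepping, with DoOnce-gated sounds on most phases.
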(event EventBeginPlay)

(event Collision|EventActorBeginOverlap
  (params (OtherActor :type Actor%20Object%20Reference)))

(event EventTick
  (params (DeltaSeconds :type Float%20%28single-precision%29))
  (bind _returnvalue (Transformation|GetActorLocation))
  (bind _returnvalue_2 (Transformation|GetActorLocation))
  (bind _returnvalue_3 (Transformation|GetActorLocation))
  (bind _returnvalue_4 (* DeltaSeconds 1e+03))
  (bind _returnvalue_5 (* DeltaSeconds 1e+03))
  (bind _returnvalue_6 (* DeltaSeconds 1e+03))
  (bind _returnvalue_7 (* DeltaSeconds 1e+03))
  (bind _returnvalue_8 (* DeltaSeconds 1e+03))
  (bind _cube (Variables|Default|GetCube))
  (bind _cube_2 (Variables|Default|GetCube))
  (bind _returnvalue_9 (+ (.z _returnvalue_3) _returnvalue_7))
  (bind _returnvalue_10 (- (.z _returnvalue_2) _returnvalue_5))
  (bind _returnvalue_11 (+ (.z _returnvalue) _returnvalue_8))
  (bind _relativelocation (Variables|/Script/Engine.SceneComponent|GetRelativeLocation _cube))
  (bind _relativelocation_2 (Variables|/Script/Engine.SceneComponent|GetRelativeLocation _cube_2))
  (bind _returnvalue_12 (- (.z _relativelocation_2) _returnvalue_6))
  (bind _returnvalue_13 (+ (.z _relativelocation) _returnvalue_4))
  (Utilities|FlowControl|Sequence
    (:then_0
      (if (Variables|Default|Getcreating)
        (if (> _returnvalue_9 125.0)
          (Variables|Default|Setcreating false)
          (Variables|Default|Setplayer%20into true)
          (else
            (Transformation|SetActorLocation (Math|Vector|MakeVector (.x _returnvalue_3) (.y _returnvalue_3) _returnvalue_9) false false)
            (Utilities|FlowControl|DoOnce false
              (:Completed
                (Audio|PlaySound2D "/Game/Sounds/BoardLevel/SW_Spawn_Pipe.SW_Spawn_Pipe" 1.0 1.0 0.0 0 0)))))))
    (:then_1
      (if (Variables|Default|Getplayer%20into)
        (if (< _returnvalue_12 0.0)
          (Variables|Default|Setplayer%20into false)
          (bind _asgm_board_game (Utilities|Casting|CastToGM_BoardGame (Game|GetGameMode)))
          (Default|SetCameraTargettoPipeSelectedNumber _asgm_board_game)
          (Default|PipeWarp _asgm_board_game (Variables|Default|Getwho%20Player?))
          (Variables|Default|Setwarp%20creating true)
          (else
            (Transformation|SetRelativeLocation _cube_2 (Math|Vector|MakeVector (.x _relativelocation_2) (.y _relativelocation_2) _returnvalue_12) false false)
            (Utilities|FlowControl|DoOnce false
              (:Completed
                (Audio|PlaySound2D "/Game/Sounds/BoardLevel/SW_PIPE.SW_PIPE" 1.0 1.0 0.0 0 0)))))))
    (:then_2
      (if (Variables|Default|Getwarp%20creating)
        (if (> _returnvalue_11 125.0)
          (Variables|Default|Setwarp%20creating false)
          (Variables|Default|Setspawn%20player true)
          (bind _asgm_board_game_2 (Utilities|Casting|CastToGM_BoardGame (Game|GetGameMode)))
          (Default|ShowPlayerinPipe _asgm_board_game_2 (Variables|Default|Getwho%20Player?))
          (else
            (Transformation|SetActorLocation (Math|Vector|MakeVector (.x _returnvalue) (.y _returnvalue) _returnvalue_11) false false)
            (Utilities|FlowControl|DoOnce false
              (:Completed
                (Audio|PlaySound2D "/Game/Sounds/BoardLevel/SW_Spawn_Pipe.SW_Spawn_Pipe" 1.0 1.0 0.0 0 0)))))))
    (:then_3
      (if (Variables|Default|Getspawn%20player)
        (if (> _returnvalue_13 4.5e+02)
          (Variables|Default|Setspawn%20player false)
          (Variables|Default|Setdisappear%20actor true)
          (else
            (Transformation|SetRelativeLocation _cube (Math|Vector|MakeVector (.x _relativelocation) (.y _relativelocation) _returnvalue_13) false false)))))
    (:then_4
      (if (Variables|Default|Getdisappear%20actor)
        (if (< _returnvalue_10 -5e+02)
          (Actor|DestroyActor)
          (bind _asgm_board_game_3 (Utilities|Casting|CastToGM_BoardGame (Game|GetGameMode)))
          (Default|FinishPipe _asgm_board_game_3 (Variables|Default|Getwho%20Player?))
          (else
            (Transformation|SetActorLocation (Math|Vector|MakeVector (.x _returnvalue_2) (.y _returnvalue_2) _returnvalue_10) false false)
            (Utilities|FlowControl|DoOnce false
              (:Completed
                (Audio|PlaySound2D "/Game/Sounds/BoardLevel/SW_PIPE.SW_PIPE" 1.0 1.0 0.0 0 0)))))))))

(fn ConstructionScript)