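; Board game player character that tracks a player's coins and stars and is colored by player number.
; The construction script picks a mesh material for the first or second player, and BeginPlay sets the board AI controller class.
; Coin and star changes are clamped, then pushed to the board game UI through the game state.
; Events stop and restart the AI controller's brain logic, while a leftover board-stepping move is never run.
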(event Custom|LogicStop
  (AI|Logic|StopLogic (Variables|/Script/AIModule.AIController|GetBrainComponent (AI|GetAIController self)) ""))

(event Custom|LogicRestart
  (Class|BrainComponent|RestartLogic (Variables|/Script/AIModule.AIController|GetBrainComponent (AI|GetAIController self))))

(event Custom|Add%20Player%20Star
  (params (Change%20Value :type Integer))
  (Variables|Default|SetStar%20Count (Math|Integer|Clamp(Integer) (+ (Variables|Default|GetStar%20Count) Change%20Value) 0 99))
  (CallFunction|SetPlayerUI))

(event Custom|Add%20Player%20Coin
  (params (Change%20Value :type Integer))
  (Variables|Default|SetCoin%20Count (Math|Integer|Clamp(Integer) (+ (Variables|Default|GetCoin%20Count) Change%20Value) 0 99))
  (CallFunction|SetPlayerUI))

(event Custom|Set%20Player%20UI
  (bind _asgs_board_game (Utilities|Casting|CastToGS_BoardGame (Game|GetGameState)))
  (Default|SetPlayerUI (Variables|/Game/BoardGame/Core/GS_BoardGame.GS_BoardGame_C|GetBoardGameUI _asgs_board_game) (Variables|Default|GetPlayerNumber) (Variables|Default|GetCoin%20Count) (Variables|Default|GetStar%20Count)))

(event EventBeginPlay
  (Variables|Default|SetAIControllerClass "/Game/BoardGame/Character/BP_BoardCharacterAiContriller.BP_BoardCharacterAiContriller_C"))

(event Collision|EventActorBeginOverlap
  (params (OtherActor :type Actor%20Object%20Reference)))

(event EventTick
  (params (DeltaSeconds :type Float%20%28single-precision%29)))

(event Input|KeyboardEvents|1
  (params (Key :type Key%20Structure :default "None")))

(fn ConstructionScript
  (switch int (Variables|Default|GetPlayerNumber)
    (:0
      (Rendering|Material|SetMaterial (Variables|Character|GetMesh) 0 "/Game/Characters/ttt/MI_1stPlayer.MI_1stPlayer"))
    (:1
      (Rendering|Material|SetMaterial (Variables|Character|GetMesh) 0 "/Game/Characters/ttt/MI_2ndPlayer.MI_2ndPlayer"))))