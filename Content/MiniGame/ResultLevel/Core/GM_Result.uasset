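; GM_Result is the game mode for the minigame result level, showing the result screen and then moving the game on.
; On BeginPlay it adds WBP_Result to the viewport and, after a delay, awards the GI_MainGame winner bonus coins and updates the widget.
; After another delay it removes player 1's controller and pawn, then opens the finish level if the turn limit is exceeded, otherwise the board game level.
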(event EventBeginPlay
  (bind _returnvalue (Game|GetPlayerController 1))
  (bind _returnvalue_2 (UserInterface|CreateWidget "/Game/MiniGame/ResultLevel/UI/WBP_Result.WBP_Result_C"))
  (bind _output_get (Variables|Default|SetResult%20UI _returnvalue_2))
  (UserInterface|Viewport|AddtoViewport _output_get 0)
  (Utilities|FlowControl|Delay 3.0)
  (bind _asgi_main_game (Utilities|Casting|CastToGI_MainGame (Game|GetGameInstance)))
  (if (!= (Variables|/Game/BoardGame/Core/GI_MainGame.GI_MainGame_C|GetWinner%20Player _asgi_main_game) -1)
    (Utilities|Array|SetArrayElem (Variables|/Game/BoardGame/Core/GI_MainGame.GI_MainGame_C|GetPlayers%20Coin _asgi_main_game) (Variables|/Game/BoardGame/Core/GI_MainGame.GI_MainGame_C|GetWinner%20Player _asgi_main_game) (+ (Utilities|Array|Get(acopy) (Variables|/Game/BoardGame/Core/GI_MainGame.GI_MainGame_C|GetPlayers%20Coin _asgi_main_game) (Variables|/Game/BoardGame/Core/GI_MainGame.GI_MainGame_C|GetWinner%20Player _asgi_main_game)) 10))
    (Default|SetWinnerCoin (Variables|Default|GetResult%20UI)))
  (Utilities|FlowControl|Delay 3.0)
  (Utilities|IsValid _returnvalue
    (:Is%20Valid
      (Class|GameplayStatics|RemovePlayer _returnvalue true))
    (:Is%20Not%20Valid
      _))
  (bind _asgi_main_game_2 (Utilities|Casting|CastToGI_MainGame (Game|GetGameInstance)))
  (if (> (Variables|/Game/BoardGame/Core/GI_MainGame.GI_MainGame_C|GetNow%20Game%20Turn _asgi_main_game_2) (Variables|/Game/BoardGame/Core/GI_MainGame.GI_MainGame_C|GetMax%20Game%20Turn _asgi_main_game_2))
    (Game|OpenLevel(byObjectReference) "/Game/StartAndFinish/Finish/FinishLevel.FinishLevel")
    (else
      (Game|OpenLevel(byObjectReference) "/Game/BoardGame/BoardGameLevel.BoardGameLevel"))))

(event EventTick
  (params (DeltaSeconds :type Float%20%28single-precision%29)))

(fn ConstructionScript)