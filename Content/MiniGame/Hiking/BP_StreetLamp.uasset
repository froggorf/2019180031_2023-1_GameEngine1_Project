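; BP_StreetLamp is a Hiking minigame actor that lays out a row of street lamps along a straight incline.
; Its construction script loops from zero through LampCount inclusive, adding a collision-free static mesh at fixed steps along local X and Z.
; Each mesh gets a point light above it with a set attenuation radius.
; The event graph holds only disabled stubs, so the actor has no runtime logic.
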(event EventBeginPlay)

(event Collision|EventActorBeginOverlap
  (params (OtherActor :type Actor%20Object%20Reference)))

(event EventTick
  (params (DeltaSeconds :type Float%20%28single-precision%29)))

(fn ConstructionScript
  (for _index (range 0 (Variables|Default|GetLamp%20Count))
    (bind _returnvalue (AddComponent|AddStaticMeshComponent false (Math|Transform|MakeTransform (Math|Vector|MakeVector (Math|Conversions|ToFloat(Integer) (* _index 2000)) 0.0 (Math|Conversions|ToFloat(Integer) (* _index 355))) "0, 0, 0" "1.000000,1.000000,1.000000")))
    (Collision|SetCollisionEnabled _returnvalue "NoCollision")
    (bind _returnvalue_2 (AddComponent|AddPointLightComponent false (Math|Transform|MakeTransform (+ (Math|Vector|MakeVector (Math|Conversions|ToFloat(Integer) (* _index 2000)) 0.0 (Math|Conversions|ToFloat(Integer) (* _index 355))) "0.000000,0.000000,425.000000") "0, 0, 0" "1.000000,1.000000,1.000000")))
    (Rendering|Lighting|SetAttenuationRadius _returnvalue_2 2.5e+03)))