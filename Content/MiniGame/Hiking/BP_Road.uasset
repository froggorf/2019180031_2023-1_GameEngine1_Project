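; BP_Road is the procedurally built uphill road for the Hiking minigame, which throws sparks where a car hits it.
; The construction script adds static mesh segments based on RoadCount, offsetting each forward and upward into a continuous slope and storing them in Roads.
; BeginPlay binds every segment's component hit event to one handler, which spawns BP_Spark at the impact point when the other actor is a BP_Car.
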(event Custom|Road%20Hit%20Event
  (params (HitComponent :type Primitive%20Component%20Object%20Reference) (OtherActor :type Actor%20Object%20Reference) (OtherComp :type Primitive%20Component%20Object%20Reference) (NormalImpulse :type Vector) (Hit :type Hit%20Result%20Structure%20%28by%20ref%29))
  (Utilities|Casting|CastToBP_Car OtherActor)
  (Game|SpawnActorfromClass "/Game/MiniGame/Hiking/Car/BP_Spark.BP_Spark_C" (Math|Transform|MakeTransform (.Location (Collision|BreakHitResult Hit)) "0, 0, 0" "1.000000,1.000000,1.000000") "Undefined" 0 0))

(event EventBeginPlay
  (for _array_element (Variables|Default|GetRoads)
    (Collision|BindEventtoOnComponentHit _array_element (delegate Custom|Road%20Hit%20Event))))

(event Collision|EventActorBeginOverlap
  (params (OtherActor :type Actor%20Object%20Reference)))

(event EventTick
  (params (DeltaSeconds :type Float%20%28single-precision%29)))

(fn ConstructionScript
  (for _index (range 0 (Variables|Default|GetRoad%20Count))
    (bind _returnvalue (AddComponent|AddStaticMeshComponent false (Math|Transform|MakeTransform (Math|Vector|MakeVector (Math|Conversions|ToFloat(Integer) (* _index 2350)) 0.0 (Math|Conversions|ToFloat(Integer) (* _index 415))) "10.000000,0.000000,0.000000" "2.000000,2.000000,2.000000")))
    (Utilities|Array|Add (Variables|Default|GetRoads) _returnvalue)))