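; BP_PlayerLine is a ground marker for the hiking minigame that shows the furthest X distance reached by the character with its PlayerNumber.
; Each Tick it moves only when that character passes it, then snaps to the surface below with a downward line trace.
; After each advance of over 10 units, it updates the distance text through GM_Hiking's UI.
; Its construction script tints the line's material for nonzero player numbers.
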(event EventBeginPlay
  (bind _outactors (Actor|GetAllActorsOfClass "/Game/MiniGame/Hiking/BP_CharacterForHiking.BP_CharacterForHiking_C"))
  (for _array_element _outactors
    (if (== (Variables|/Game/MiniGame/Hiking/BP_CharacterForHiking.BP_CharacterForHiking_C|GetPlayerNumber _array_element) (Variables|Default|GetPlayer%20Number))
      (Variables|Default|SetMy%20Character _array_element))))

(event Collision|EventActorBeginOverlap
  (params (OtherActor :type Actor%20Object%20Reference)))

(event EventTick
  (params (DeltaSeconds :type Float%20%28single-precision%29))
  (bind _returnvalue (Transformation|GetActorLocation))
  (bind _returnvalue_2 (Transformation|GetActorLocation))
  (bind _my_character (Variables|Default|GetMy%20Character))
  (bind _returnvalue_3 (Transformation|GetActorLocation _my_character))
  (if (< (.x (Transformation|GetActorLocation)) (.x _returnvalue_3))
    (Transformation|SetActorLocation (Math|Vector|MakeVector (.x _returnvalue_3) 0.0 (.z _returnvalue_3)) false false)
    (bind _outhit (Collision|LineTraceByChannel _returnvalue_2 (+ _returnvalue_2 "0.000000,0.000000,-10000.000000") "TraceTypeQuery1" false 0 "None"))
    (Transformation|SetActorLocation (.Location (Collision|BreakHitResult _outhit)) false false)
    (if (> (- (.x (Transformation|GetActorLocation)) (Variables|Default|Getlast%20distance)) 1e+01)
      (bind _asgm_hiking (Utilities|Casting|CastToGM_Hiking (Game|GetGameMode)))
      (Default|SetDistanceText (Variables|/Game/MiniGame/Hiking/core/GM_Hiking.GM_Hiking_C|GetHikingGame%20UI _asgm_hiking) (Variables|Default|GetPlayer%20Number) (.x _returnvalue))
      (Variables|Default|Setlast%20distance (.x _returnvalue)))))

(fn ConstructionScript
  (bind _returnvalue (Rendering|Material|CreateDynamicMaterialInstance (Variables|Default|GetCylinder) 0 "/Game/MiniGame/Hiking/M_PlayerLine.M_PlayerLine" "None" :!class /Script/Engine.PrimitiveComponent))
  (if (not (== (Variables|Default|GetPlayer%20Number) 0))
    (Rendering|Material|SetVectorParameterValue _returnvalue "Color" "(R=0.000000,G=0.134427,B=1.000000,A=1.000000)" :!class /Script/Engine.MaterialInstanceDynamic)))