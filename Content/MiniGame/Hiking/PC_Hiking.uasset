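; Player controller for the hiking minigame that handles movement, jumping and camera look.
; On BeginPlay it adds the IMC_Hiking Enhanced Input mapping context.
; Move input drives the controlled pawn along its control rotation's forward and right vectors, and mouse input adds yaw and pitch.
; The space action calls Jump on the pawn after casting it to BP_CharacterForHiking.
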(event Input|EnhancedActionEvents|EnhancedInputActionIA_MoveForHiking
  (params (ActionValue :type Vector%202D%20Structure) (ElapsedSeconds :type Float%20%28double-precision%29) (TriggeredSeconds :type Float%20%28double-precision%29) (InputAction :type Input%20Action%20Object%20Reference :default "/Game/MiniGame/Hiking/Input/IA_MoveForHiking.IA_MoveForHiking"))
  (bind _returnvalue (Pawn|GetControlledPawn))
  (bind _returnvalue_2 (Pawn|GetControlRotation _returnvalue :!class /Script/Engine.Pawn))
  (:Triggered
    (Pawn|Input|AddMovementInput _returnvalue (Math|Vector|GetForwardVector _returnvalue_2) (.x ActionValue) false)
    (Pawn|Input|AddMovementInput _returnvalue (Math|Vector|GetRightVector _returnvalue_2) (.y ActionValue) false)))

(event Input|EnhancedActionEvents|EnhancedInputActionIA_SpaceForHiking
  (params (ActionValue :type Boolean) (ElapsedSeconds :type Float%20%28double-precision%29) (TriggeredSeconds :type Float%20%28double-precision%29) (InputAction :type Input%20Action%20Object%20Reference :default "/Game/MiniGame/Hiking/Input/IA_SpaceForHiking.IA_SpaceForHiking"))
  (:Started
    (bind _asbp_character_for_hiking (Utilities|Casting|CastToBP_CharacterForHiking (Pawn|GetControlledPawn)))
    (Character|Jump _asbp_character_for_hiking)))

(event Input|EnhancedActionEvents|EnhancedInputActionIA_MouseForHiking
  (params (ActionValue :type Vector%202D%20Structure) (ElapsedSeconds :type Float%20%28double-precision%29) (TriggeredSeconds :type Float%20%28double-precision%29) (InputAction :type Input%20Action%20Object%20Reference :default "/Game/MiniGame/Hiking/Input/IA_MouseForHiking.IA_MouseForHiking"))
  (:Triggered
    (Class|PlayerController|AddYawInput (.x ActionValue))
    (Class|PlayerController|AddPitchInput (.y ActionValue))))

(event EventBeginPlay
  (Input|AddMappingContext (PlayerController|LocalPlayerSubsystems|GetEnhancedInputLocalPlayerSubsystem) "/Game/MiniGame/Hiking/Input/IMC_Hiking.IMC_Hiking" 0 "(bIgnoreAllPressedKeysUntilRelease=True,bForceImmediately=False)"))

(fn ConstructionScript)