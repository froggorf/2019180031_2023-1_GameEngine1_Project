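; Player character for the Hiking minigame that gets sent back to its start when hit by a car.
; BeginPlay stores a spawn point raised above the starting location.
; A capsule hit from a BP_Car moves the character there and zeroes its walk speed for a short delay before setting it back.
; The Construction Script assigns the first or second player's mesh material from PlayerNumber.
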(event OnComponentHit(CapsuleComponent)
  (params (HitComponent :type Primitive%20Component%20Object%20Reference) (OtherActor :type Actor%20Object%20Reference) (OtherComp :type Primitive%20Component%20Object%20Reference) (NormalImpulse :type Vector :default "0, 0, 0") (Hit :type Hit%20Result%20Structure%20%28by%20ref%29))
  (bind _charactermovement (Variables|Character|GetCharacterMovement))
  (Utilities|Casting|CastToBP_Car OtherActor)
  (Transformation|SetActorLocation (Variables|Default|GetSpawn%20Point) false false)
  (Variables|/Script/Engine.CharacterMovementComponent|SetMaxWalkSpeed _charactermovement 0.0)
  (Utilities|FlowControl|Delay 1.0)
  (Variables|/Script/Engine.CharacterMovementComponent|SetMaxWalkSpeed _charactermovement 6e+02))

(event EventBeginPlay
  (Variables|Default|SetSpawn%20Point (+ (Transformation|GetActorLocation) "0.000000,0.000000,200.000000")))

(event Collision|EventActorBeginOverlap
  (params (OtherActor :type Actor%20Object%20Reference)))

(event EventTick
  (params (DeltaSeconds :type Float%20%28single-precision%29)))

(fn ConstructionScript
  (bind _mesh (Variables|Character|GetMesh))
  (switch int (Variables|Default|GetPlayerNumber)
    (:0
      (Rendering|Material|SetMaterial _mesh 0 "/Game/MiniGame/BaseBall/Character/MI_1stPlayer.MI_1stPlayer"))
    (:1
      (Rendering|Material|SetMaterial _mesh 0 "/Game/MiniGame/BaseBall/Character/MI_2ndPlayer.MI_2ndPlayer"))))