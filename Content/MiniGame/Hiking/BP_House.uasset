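; BP_House is a construction-script Blueprint in the Hiking minigame that builds a row of static mesh components, presumably houses.
; A loop driven by HouseNumber spaces them along X and raises each one in Z, forming an ascending line.
; Even and odd indices use separate add-component nodes with identical offset math.
; The event graph holds no active logic.
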(event EventBeginPlay)

(event Collision|EventActorBeginOverlap
  (params (OtherActor :type Actor%20Object%20Reference)))

(event EventTick
  (params (DeltaSeconds :type Float%20%28single-precision%29)))

(fn ConstructionScript
  (for _index (range 0 (Variables|Default|GetHouse%20Number))
    (if (== (Math|Integer|%(Integer) _index 2) 0)
      (AddComponent|AddStaticMeshComponent false (Math|Transform|MakeTransform (Math|Vector|MakeVector (Math|Conversions|ToFloat(Integer) (* _index 620)) 0.0 (Math|Conversions|ToFloat(Integer) (* _index 110))) "0, 0, 0" "1.000000,1.000000,1.000000"))
      (else
        (AddComponent|AddStaticMeshComponent false (Math|Transform|MakeTransform (Math|Vector|MakeVector (Math|Conversions|ToFloat(Integer) (* _index 620)) 0.0 (Math|Conversions|ToFloat(Integer) (* _index 110))) "0, 0, 0" "1.000000,1.000000,1.000000"))))))