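; BP_Car is a hiking minigame car that switches into a physics-driven slide or launch on demand.
; SimulateOn and SimulatePhysicsoff toggle skeletal mesh physics along with a flag that gates Tick.
; While simulating, Tick applies a large mass-dependent impulse every frame, unscaled by delta time, along world -X and slightly downward, using a pitched vector cached at BeginPlay plus random sideways jitter.
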(event Custom|Simulate%20Physics%20off
  (Physics|SetSimulatePhysics (Variables|Default|GetSkeletalMesh) false)
  (Variables|Default|Setis%20simulated%20physics? false))

(event Custom|Simulate%20On
  (Physics|SetSimulatePhysics (Variables|Default|GetSkeletalMesh) true)
  (Variables|Default|Setis%20simulated%20physics? true))

(event EventBeginPlay
  (Variables|Default|SetNewVar_0 (Math|Vector|RotateVector (Math|Vector|MakeVector 1.0 0.0 0.0) (Math|Rotator|MakeRotator 0.0 1e+01 0.0))))

(event Collision|EventActorBeginOverlap
  (params (OtherActor :type Actor%20Object%20Reference)))

(event EventTick
  (params (DeltaSeconds :type Float%20%28single-precision%29))
  (if (Variables|Default|Getis%20simulated%20physics?)
    (Physics|AddImpulse (Variables|Default|GetSkeletalMesh) (* (+ (Variables|Default|GetNewVar_0) (Math|Vector|MakeVector 0.0 (Math|Random|RandomFloatinRange -0.5 0.5) 0.0)) "-15000.000000,-15000.000000,-30000.000000") "None" false)))

(fn ConstructionScript)