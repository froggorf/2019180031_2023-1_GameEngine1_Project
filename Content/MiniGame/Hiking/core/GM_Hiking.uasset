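; Game mode for the two-player Hiking minigame, a timed contest in which cars keep spawning and the greater distance wins.
; Tick runs a step state machine with DoOnce-guarded entries: guide until both players ready, countdown, play, finish.
; Play spawns random cars at every TargetPoint on random intervals while the timer runs down.
; Finish compares each BP_PlayerLine's LastDistance, stores winner or tie in GI_MainGame, then opens the result level.
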(event Custom|Game%20Play%20Event
  (bind _hikinggame_ui (Variables|Default|GetHikingGame%20UI))
  ;[1 1 1] Game_Play
  (Utilities|FlowControl|Sequence
    (:then_0
      (Utilities|FlowControl|DoOnce false
        (:Completed
          (bind _outactors (Actor|GetAllActorsOfClass "/Game/MiniGame/Hiking/Car/BP_Car.BP_Car_C"))
          (for _array_element _outactors
            (Default|Simulateon _array_element)))))
    (:then_1
      (if (Variables|Default|Getspawn%20car?)
        (Variables|Default|Setspawn%20car? false)
        (for _array_element_2 (Variables|Default|GetSpawn%20Car%20Locations)
          (Game|SpawnActorfromClass (.OutItem (Utilities|Array|Random (Utilities|Array|MakeArray "/Game/MiniGame/Hiking/Car/BP_Car01.BP_Car01_C" "/Game/MiniGame/Hiking/Car/BP_Car02.BP_Car02_C" "/Game/MiniGame/Hiking/Car/BP_Car03.BP_Car03_C" "/Game/MiniGame/Hiking/Car/BP_Car04.BP_Car04_C"))) (Math|Transform|MakeTransform (Transformation|GetActorLocation _array_element_2) "0, 0, 0" "1.000000,1.000000,1.000000") "Undefined" 0 0))
        (Utilities|FlowControl|Delay (Math|Random|RandomFloatinRange 1.3 2.3))
        (Variables|Default|Setspawn%20car? true)))
    (:then_2
      (Variables|Default|SetGameTime (- (Variables|Default|GetGameTime) (Utilities|Time|GetWorldDeltaSeconds)))
      (if (<= (- (Variables|Default|GetGameTime) (Utilities|Time|GetWorldDeltaSeconds)) 0.0)
        (Variables|Default|SetGameTime 0.0)
        (Default|SetTimeText _hikinggame_ui 0.0)
        (Variables|Default|SetGame%20Step "GAME_FINISH")
        (else
          (Default|SetTimeText _hikinggame_ui (Variables|Default|GetGameTime)))))))

(event Custom|Guide%20State%20Event
  ;[1 1 1] Guide State
  (Utilities|FlowControl|Sequence
    (:then_0
      (Utilities|FlowControl|DoOnce false
        (:Completed
          (bind _returnvalue (UserInterface|CreateWidget "/Game/MiniGame/Hiking/UI/WBP_GuideForHiking.WBP_GuideForHiking_C"))
          (bind _output_get (Variables|Default|SetGuideUI _returnvalue))
          (UserInterface|Viewport|AddtoViewport _output_get 0)
          (bind _aspc_hiking (Utilities|Casting|CastToPC_Hiking (Game|GetPlayerController 0)))
          (Default|StartKeyMapping _aspc_hiking))))
    (:then_1
      (if (not (Utilities|Array|ContainsItem (Variables|Default|GetPlayer%20Ready%20Check) false))
        (Utilities|FlowControl|DoOnce false
          (:Completed
            (Widget|RemovefromParent (Variables|Default|GetGuideUI))
            (Variables|Default|SetGame%20Step "GAME_START")))))))

(event Custom|Set%20Ready%20True
  (params (Player%20Number :type Integer))
  ;[1 1 1] Guide State
  (Utilities|Array|SetArrayElem (Variables|Default|GetPlayer%20Ready%20Check) Player%20Number true)
  (Default|SetPlayerReady (Variables|Default|GetGuideUI) Player%20Number))

(event Custom|Game%20Start%20Event
  ;[1 1 1] Game_Start
  (Utilities|FlowControl|Sequence
    (:then_0
      (Utilities|FlowControl|DoOnce false
        (:Completed
          (Default|TurnOffSound (Variables|Default|GetGuideUI))
          (bind _returnvalue (UserInterface|CreateWidget "/Game/MiniGame/Hiking/UI/WBP_HikingGameUI.WBP_HikingGameUI_C"))
          (bind _output_get (Variables|Default|SetHikingGame%20UI _returnvalue))
          (UserInterface|Viewport|AddtoViewport _output_get 0)
          (Utilities|FlowControl|Delay 0.5)
          (Default|SetTimeTextatStart (Variables|Default|GetHikingGame%20UI) 3)
          (Utilities|FlowControl|Delay 1.0)
          (Default|SetTimeTextatStart (Variables|Default|GetHikingGame%20UI) 2)
          (Utilities|FlowControl|Delay 1.0)
          (Default|SetTimeTextatStart (Variables|Default|GetHikingGame%20UI) 1)
          (Utilities|FlowControl|Delay 1.0)
          (Variables|/Script/UMG.TextBlock|SetText (Variables|/Game/MiniGame/Hiking/UI/WBP_HikingGameUI.WBP_HikingGameUI_C|GetTimeTextAtStart (Variables|Default|GetHikingGame%20UI)) "시작!")
          (Utilities|FlowControl|Delay 0.5)
          (Widget|SetVisibility (Variables|/Game/MiniGame/Hiking/UI/WBP_HikingGameUI.WBP_HikingGameUI_C|GetTimeTextAtStart (Variables|Default|GetHikingGame%20UI)) "Hidden")
          (Widget|SetVisibility (Variables|/Game/MiniGame/Hiking/UI/WBP_HikingGameUI.WBP_HikingGameUI_C|GetTimeText (Variables|Default|GetHikingGame%20UI)) "Visible")
          (Variables|Default|SetGameTime (Variables|Default|GetGameInitTime))
          (bind _aspc_hiking (Utilities|Casting|CastToPC_Hiking (Game|GetPlayerController 0)))
          (Default|GamePlayKeyMapping _aspc_hiking)
          (Variables|Default|SetGame%20Step "GAME_PLAY"))))))

(event Custom|Game%20Finish%20Event
  (bind _player_lines (Variables|Default|GetPlayer%20Lines))
  (bind _output (Utilities|Array|Get(acopy) _player_lines))
  (bind _output_2 (Utilities|Array|Get(acopy) _player_lines 1))
  (bind _last_distance (Variables|/Game/MiniGame/Hiking/BP_PlayerLine.BP_PlayerLine_C|Getlast%20distance _output))
  (bind _last_distance_2 (Variables|/Game/MiniGame/Hiking/BP_PlayerLine.BP_PlayerLine_C|Getlast%20distance _output_2))
  ;[1 1 1] Game Result
  (Utilities|FlowControl|DoOnce false
    (:Completed
      (bind _aspc_hiking (Utilities|Casting|CastToPC_Hiking (Game|GetPlayerController 0)))
      (Default|RemoveAllMapping _aspc_hiking)
      (Default|FinishGameUI (Variables|Default|GetHikingGame%20UI) (Utilities|Array|MakeArray _last_distance _last_distance_2))
      (bind _asgi_main_game (Utilities|Casting|CastToGI_MainGame (Game|GetGameInstance)))
      (if (== _last_distance _last_distance_2)
        (Variables|/Game/BoardGame/Core/GI_MainGame.GI_MainGame_C|SetWinner%20Player _asgi_main_game -1)
        (elif (> _last_distance _last_distance_2)
          (Variables|/Game/BoardGame/Core/GI_MainGame.GI_MainGame_C|SetWinner%20Player _asgi_main_game 0)
          (else
            (Variables|/Game/BoardGame/Core/GI_MainGame.GI_MainGame_C|SetWinner%20Player _asgi_main_game 1))))
      (Utilities|FlowControl|Delay 3.0)
      (Game|OpenLevel(byObjectReference) "/Game/MiniGame/ResultLevel/ResultLevel.ResultLevel"))))

(event Custom|DEBUG_CHANGE_GAME
  (Game|OpenLevel(byObjectReference) "/Game/MiniGame/BaseBall/BaseBallMap.BaseBallMap"))

(event EventBeginPlay
  ;[1 1 1] Begin Play
  (Class|GameplayStatics|CreatePlayer 0)
  (Class|GameplayStatics|CreatePlayer 1)
  (bind _outactors (Actor|GetAllActorsOfClass "/Script/Engine.TargetPoint"))
  (Variables|Default|SetSpawn%20Car%20Locations _outactors)
  (bind _outactors_2 (Actor|GetAllActorsOfClass "/Game/MiniGame/Hiking/BP_PlayerLine.BP_PlayerLine_C"))
  (CallFunction|GetPlayerLine _outactors_2)
  (bind _outactors_3 (Actor|GetAllActorsOfClass "/Game/MiniGame/Hiking/Car/BP_Car.BP_Car_C"))
  (for _array_element _outactors_3
    (Default|SimulatePhysicsOff _array_element))
  (Variables|Default|SetGame%20Step "GUIDE_STATE"))

(event EventTick
  (params (DeltaSeconds :type Float%20%28single-precision%29))
  ;[1 1 1] Main
  (switch string (Variables|Default|GetGame%20Step)
    (:GUIDE_STATE
      (CallFunction|GuideStateEvent))
    (:GAME_START
      (CallFunction|GameStartEvent))
    (:GAME_PLAY
      (CallFunction|GamePlayEvent))
    (:GAME_FINISH
      (CallFunction|GameFinishEvent))))

(fn ConstructionScript)

(fn GetPlayerLine
  (params (NewParam :type Array%20of%20BP%20Player%20Line%20Object%20References))
  (for _array_element NewParam :!label _label
    (if (== (Utilities|Array|Length (Variables|Default|GetPlayer%20Lines)) (Variables|/Game/MiniGame/Hiking/BP_PlayerLine.BP_PlayerLine_C|GetPlayer%20Number _array_element))
      (Utilities|Array|Add (Variables|Default|GetPlayer%20Lines) _array_element)
      (goto _label))))