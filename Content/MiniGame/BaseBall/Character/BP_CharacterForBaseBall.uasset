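; BP_CharacterForBaseBall is the baseball minigame character that swings and throws a bat.
; BatHit plays the BaseBallHit section of the AM_Baseball montage behind a DoOnce, then re-shows the held bat mesh and resets when the montage completes.
; ReleaseBat hides that mesh, disables its collision, then spawns a BP_Bat at its transform and throws it along the hand socket's up vector.
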(event Custom|Bat%20Hit
  (Utilities|FlowControl|DoOnce false :!label _label
    (:Completed
      (Animation|Montage|PlayMontage (Variables|Character|GetMesh) "/Game/MiniGame/BaseBall/Character/AM_Baseball.AM_Baseball" 1.0 0.0 "BaseBallHit"
        (:OnCompleted
          (Rendering|SetVisibility (Variables|Default|GetSM_Test) true false)
          (goto _label Reset))))))

(event Custom|Release%20Bat
  (bind _sm_test (Variables|Default|GetSM_Test))
  (bind _returnvalue (Transformation|GetWorldTransform _sm_test))
  (Rendering|SetVisibility _sm_test false false)
  (Collision|SetCollisionEnabled _sm_test "NoCollision")
  (bind _returnvalue_2 (Game|SpawnActorfromClass "/Game/MiniGame/BaseBall/BP_Bat.BP_Bat_C" (Math|Transform|MakeTransform (.location _returnvalue) (.rotation _returnvalue) (.scale _returnvalue)) "Undefined" 0 0))
  (Default|Throw _returnvalue_2 (* (Math|Vector|GetUpVector (.rotation (Transformation|GetSocketTransform (Variables|Character|GetMesh) "BatSocket" "RTS_World"))) 5e+04)))

(event EventBeginPlay)

(event Collision|EventActorBeginOverlap
  (params (OtherActor :type Actor%20Object%20Reference)))

(event EventTick
  (params (DeltaSeconds :type Float%20%28single-precision%29)))

(fn ConstructionScript)