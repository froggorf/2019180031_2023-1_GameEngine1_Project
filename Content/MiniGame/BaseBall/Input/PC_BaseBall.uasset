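; Player controller for the baseball minigame, handling two players' input from a single controller through Enhanced Input.
; During the guide, Space and Right Shift each mark player 0 or 1 ready in GM_BaseBall, once only.
; GamePlayKeyMapping then swaps the guide mapping context for the baseball one.
; In play, Space calls BatHit on the controlled pawn and Right Shift on player character 1.
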(event Custom|Set%20Player%20Guide%20Mapping
  ;[1 1 1] Guide Input Action
  (Input|AddMappingContext (PlayerController|LocalPlayerSubsystems|GetEnhancedInputLocalPlayerSubsystem self) "/Game/MiniGame/BaseBall/Input/GuideUIInput/IMC_GuideForBaseBall.IMC_GuideForBaseBall" 0 "(bIgnoreAllPressedKeysUntilRelease=True,bForceImmediately=False)"))

(event Custom|Remove%20All%20Mapping
  (bind _self self)
  (bind _returnvalue (PlayerController|LocalPlayerSubsystems|GetEnhancedInputLocalPlayerSubsystem _self))
  (Input|RemoveMappingContext _returnvalue "/Game/MiniGame/BaseBall/Input/BaseBallGameStart/IMC_Baseball.IMC_Baseball" "(bIgnoreAllPressedKeysUntilRelease=True,bForceImmediately=False)")
  (Input|RemoveMappingContext _returnvalue "/Game/MiniGame/BaseBall/Input/GuideUIInput/IMC_GuideForBaseBall.IMC_GuideForBaseBall" "(bIgnoreAllPressedKeysUntilRelease=True,bForceImmediately=False)"))

(event Custom|Game%20Play%20Key%20Mapping
  ;[1 1 1] Game Play Key Mapping
  (CallFunction|RemoveAllMapping)
  (Input|AddMappingContext (PlayerController|LocalPlayerSubsystems|GetEnhancedInputLocalPlayerSubsystem self) "/Game/MiniGame/BaseBall/Input/BaseBallGameStart/IMC_Baseball.IMC_Baseball" 0 "(bIgnoreAllPressedKeysUntilRelease=True,bForceImmediately=False)"))

(event Input|EnhancedActionEvents|EnhancedInputActionIA_SpaceForBaseball
  (params (ActionValue :type Boolean) (ElapsedSeconds :type Float%20%28double-precision%29) (TriggeredSeconds :type Float%20%28double-precision%29) (InputAction :type Input%20Action%20Object%20Reference :default "/Game/MiniGame/BaseBall/Input/BaseBallGameStart/IA_SpaceForBaseball.IA_SpaceForBaseball"))
  ;[1 1 1] Game Play Key Mapping
  (:Triggered
    (bind _asbp_character_for_base_ball (Utilities|Casting|CastToBP_CharacterForBaseBall (Pawn|GetControlledPawn)))
    (Default|BatHit _asbp_character_for_base_ball)))

(event Input|EnhancedActionEvents|EnhancedInputActionIA_RShiftForBaseball
  (params (ActionValue :type Boolean) (ElapsedSeconds :type Float%20%28double-precision%29) (TriggeredSeconds :type Float%20%28double-precision%29) (InputAction :type Input%20Action%20Object%20Reference :default "/Game/MiniGame/BaseBall/Input/BaseBallGameStart/IA_RShiftForBaseball.IA_RShiftForBaseball"))
  ;[1 1 1] Game Play Key Mapping
  (:Started
    (bind _asbp_character_for_base_ball (Utilities|Casting|CastToBP_CharacterForBaseBall (Game|GetPlayerCharacter 1)))
    (Default|BatHit _asbp_character_for_base_ball)))

(event Input|EnhancedActionEvents|EnhancedInputActionIA_SpaceForGuide
  (params (ActionValue :type Boolean) (ElapsedSeconds :type Float%20%28double-precision%29) (TriggeredSeconds :type Float%20%28double-precision%29) (InputAction :type Input%20Action%20Object%20Reference :default "/Game/MiniGame/BaseBall/Input/GuideUIInput/IA_SpaceForGuide.IA_SpaceForGuide"))
  ;[1 1 1] Guide Input Action
  (:Started
    (Utilities|FlowControl|DoOnce false
      (:Completed
        (bind _asgm_base_ball (Utilities|Casting|CastToGM_BaseBall (Game|GetGameMode)))
        (Default|SetReadyTrue _asgm_base_ball)))))

(event Input|EnhancedActionEvents|EnhancedInputActionIA_RSHIFTForGuide
  (params (ActionValue :type Boolean) (ElapsedSeconds :type Float%20%28double-precision%29) (TriggeredSeconds :type Float%20%28double-precision%29) (InputAction :type Input%20Action%20Object%20Reference :default "/Game/MiniGame/BaseBall/Input/GuideUIInput/IA_RSHIFTForGuide.IA_RSHIFTForGuide"))
  ;[1 1 1] Guide Input Action
  (:Started
    (Utilities|FlowControl|DoOnce false
      (:Completed
        (bind _asgm_base_ball (Utilities|Casting|CastToGM_BaseBall (Game|GetGameMode)))
        (Default|SetReadyTrue _asgm_base_ball 1)))))

(event EventTick
  (params (DeltaSeconds :type Float%20%28single-precision%29)))

(fn ConstructionScript)