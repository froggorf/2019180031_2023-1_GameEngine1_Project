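; Game mode for a local two-player baseball minigame in which players score hits on spawned balls before time runs out.
; Tick runs a step machine: guide video until both players are ready, countdown, timed play, then finish.
; During play it spawns a ball above each player at random intervals and relays hit counts to the HUD.
; At the finish it stores the winner or a tie in GI_MainGame and opens the result level.
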(event Custom|DEBUG_CHANGE_GAME
  (Game|OpenLevel(byObjectReference) "/Game/MiniGame/Hiking/HikingMap.HikingMap"))

(event Custom|Guide_State
  ;[1 1 1] Guide State
  (Utilities|FlowControl|Sequence
    (:then_0
      (Utilities|FlowControl|DoOnce false
        (:Completed
          (bind _returnvalue (UserInterface|CreateWidget "/Game/MiniGame/BaseBall/core/UI/WBP_VideoUIForBaseBallMAp.WBP_VideoUIForBaseBallMAp_C"))
          (bind _output_get (Variables|Default|SetBaseBall%20Guide%20UI _returnvalue))
          (UserInterface|Viewport|AddtoViewport _output_get 0)
          (bind _aspc_base_ball (Utilities|Casting|CastToPC_BaseBall (Game|GetPlayerController 0)))
          (Default|SetPlayerGuideMapping _aspc_base_ball))))
    (:then_1
      (if (not (Utilities|Array|ContainsItem (Variables|Default|GetPlayer%20Ready%20Check) false))
        (Utilities|FlowControl|DoOnce false
          (:Completed
            (Widget|RemovefromParent (Variables|Default|GetBaseBall%20Guide%20UI))
            (Default|TurnOffSound (Variables|Default|GetBaseBall%20Guide%20UI))
            (Variables|Default|SetGameStep "GAME_START")))))))

(event Custom|Game%20Finish%20Event
  (bind _players (Variables|Default|Getplayers))
  (bind _output (Utilities|Array|Get(acopy) _players))
  (bind _output_2 (Utilities|Array|Get(acopy) _players 1))
  (bind _hit_count (Variables|/Game/MiniGame/BaseBall/Character/BP_CharacterForBaseBall.BP_CharacterForBaseBall_C|GetHit%20Count _output_2))
  (bind _hit_count_2 (Variables|/Game/MiniGame/BaseBall/Character/BP_CharacterForBaseBall.BP_CharacterForBaseBall_C|GetHit%20Count _output))
  (Utilities|FlowControl|Sequence
    (:then_0
      (Utilities|FlowControl|DoOnce false
        (:Completed
          (bind _aspc_base_ball (Utilities|Casting|CastToPC_BaseBall (Game|GetPlayerController 0)))
          (Default|RemoveAllMapping _aspc_base_ball)
          (Default|FinishGameUI (Variables|Default|GetBaseBall%20Play%20UI) (Utilities|Array|MakeArray _hit_count_2 _hit_count))
          (bind _asgi_main_game (Utilities|Casting|CastToGI_MainGame (Game|GetGameInstance)))
          (if (== _hit_count_2 _hit_count)
            (Variables|/Game/BoardGame/Core/GI_MainGame.GI_MainGame_C|SetWinner%20Player _asgi_main_game -1)
            (elif (> _hit_count_2 _hit_count)
              (Variables|/Game/BoardGame/Core/GI_MainGame.GI_MainGame_C|SetWinner%20Player _asgi_main_game 0)
              (else
                (Variables|/Game/BoardGame/Core/GI_MainGame.GI_MainGame_C|SetWinner%20Player _asgi_main_game 1))))
          (Utilities|FlowControl|Delay 3.0)
          (Game|OpenLevel(byObjectReference) "/Game/MiniGame/ResultLevel/ResultLevel.ResultLevel"))))))

(event Custom|Set%20Ready%20True
  (params (Player%20Number :type Integer))
  ;[1 1 1] Guide State
  (Utilities|Array|SetArrayElem (Variables|Default|GetPlayer%20Ready%20Check) Player%20Number true)
  (Default|SetPlayerReady (Variables|Default|GetBaseBall%20Guide%20UI) Player%20Number))

(event Custom|Game%20Start%20Event
  ;[1 1 1] Game Start
  (Utilities|FlowControl|Sequence
    (:then_0
      (Utilities|FlowControl|DoOnce false
        (:Completed
          (bind _returnvalue (UserInterface|CreateWidget "/Game/MiniGame/BaseBall/core/UI/WBP_BaseBallGamePlay.WBP_BaseBallGamePlay_C"))
          (bind _output_get (Variables|Default|SetBaseBall%20Play%20UI _returnvalue))
          (UserInterface|Viewport|AddtoViewport _output_get 0)
          (Utilities|FlowControl|Delay 0.5)
          (Default|SetTimeTextatStart (Variables|Default|GetBaseBall%20Play%20UI) 3)
          (Utilities|FlowControl|Delay 1.0)
          (Default|SetTimeTextatStart (Variables|Default|GetBaseBall%20Play%20UI) 2)
          (Utilities|FlowControl|Delay 1.0)
          (Default|SetTimeTextatStart (Variables|Default|GetBaseBall%20Play%20UI) 1)
          (Utilities|FlowControl|Delay 1.0)
          (Variables|/Script/UMG.TextBlock|SetText (Variables|/Game/MiniGame/BaseBall/core/UI/WBP_BaseBallGamePlay.WBP_BaseBallGamePlay_C|GetTimeTextAtStart (Variables|Default|GetBaseBall%20Play%20UI)) "시작!")
          (Utilities|FlowControl|Delay 0.5)
          (Widget|SetVisibility (Variables|/Game/MiniGame/BaseBall/core/UI/WBP_BaseBallGamePlay.WBP_BaseBallGamePlay_C|Gettimetextatstartborder (Variables|Default|GetBaseBall%20Play%20UI)) "Hidden")
          (Widget|SetVisibility (Variables|/Game/MiniGame/BaseBall/core/UI/WBP_BaseBallGamePlay.WBP_BaseBallGamePlay_C|Gettimetextborder (Variables|Default|GetBaseBall%20Play%20UI)) "Visible")
          (Variables|Default|SetGame%20Time (Variables|Default|GetGame%20Init%20Time))
          (bind _aspc_base_ball (Utilities|Casting|CastToPC_BaseBall (Game|GetPlayerController 0)))
          (Default|GamePlayKeyMapping _aspc_base_ball)
          (Variables|Default|SetGameStep "GAME_PLAY"))))))

(event Custom|Game%20Play
  (bind _baseball_play_ui (Variables|Default|GetBaseBall%20Play%20UI))
  ;[1 1 1] Game Play
  (Utilities|FlowControl|Sequence
    (:then_0
      (if (Variables|Default|GetSpawn%20Ball)
        (Variables|Default|SetSpawn%20Ball false)
        (for (_array_element _array_index) (Variables|Default|Getplayers)
          (bind _returnvalue (Game|SpawnActorfromClass "/Game/MiniGame/BaseBall/BP_Ball.BP_Ball_C" (Math|Transform|MakeTransform (+ (Transformation|GetWorldLocation (Variables|/Game/MiniGame/BaseBall/Character/BP_CharacterForBaseBall.BP_CharacterForBaseBall_C|GetSpringArm _array_element)) "15.000000,0.000000,500.000000") "0, 0, 0" "1.000000,1.000000,1.000000") "Undefined" 0 0))
          (Default|SetPlayerNumber _returnvalue _array_index))
        (Utilities|FlowControl|Delay (Math|Random|RandomFloatinRange 1.5 2.0))
        (Variables|Default|SetSpawn%20Ball true)))
    (:then_1
      (Variables|Default|SetGame%20Time (- (Variables|Default|GetGame%20Time) (Utilities|Time|GetWorldDeltaSeconds)))
      (if (<= (- (Variables|Default|GetGame%20Time) (Utilities|Time|GetWorldDeltaSeconds)) 0.0)
        (Variables|Default|SetGame%20Time 0.0)
        (Default|SetTimeText _baseball_play_ui 0.0)
        (Variables|Default|SetGameStep "GAME_FINISH")
        (else
          (Default|SetTimeText _baseball_play_ui (Variables|Default|GetGame%20Time)))))))

(event Custom|Player%20Get%20Score
  (params (Player%20Number :type Integer))
  (bind _players (Variables|Default|Getplayers))
  (bind _output (Utilities|Array|Get(acopy) _players Player%20Number))
  (bind _output_get (Variables|/Game/MiniGame/BaseBall/Character/BP_CharacterForBaseBall.BP_CharacterForBaseBall_C|SetHit%20Count _output (+ (Variables|/Game/MiniGame/BaseBall/Character/BP_CharacterForBaseBall.BP_CharacterForBaseBall_C|GetHit%20Count _output) 1)))
  (Default|SetScoreText (Variables|Default|GetBaseBall%20Play%20UI) Player%20Number _output_get))

(event EventBeginPlay
  ;[1 1 1] Begin Play
  (Class|GameplayStatics|CreatePlayer 0)
  (Class|GameplayStatics|CreatePlayer 1)
  (bind _outactors (Actor|GetAllActorsOfClass "/Game/MiniGame/BaseBall/Character/BP_CharacterForBaseBall.BP_CharacterForBaseBall_C"))
  (CallFunction|GetPlayerArray _outactors)
  (Variables|Default|SetGameStep "GUIDE_STATE"))

(event EventTick
  (params (DeltaSeconds :type Float%20%28single-precision%29))
  ;[1 1 1] Main
  (switch string (Variables|Default|GetGameStep)
    (:GUIDE_STATE
      (CallFunction|GuideState))
    (:GAME_START
      (CallFunction|GameStartEvent))
    (:GAME_PLAY
      (CallFunction|GamePlay))
    (:GAME_FINISH
      (CallFunction|GameFinishEvent))))

(fn ConstructionScript)

(fn GetPlayerArray
  (params (characters :type Array%20of%20BP%20Character%20for%20Base%20Ball%20Object%20References))
  (for _array_element characters :!label _label
    (if (== (Variables|/Game/MiniGame/BaseBall/Character/BP_CharacterForBaseBall.BP_CharacterForBaseBall_C|GetPlayer%20Number _array_element) (Utilities|Array|Length (Variables|Default|Getplayers)))
      (Utilities|Array|Add (Variables|Default|Getplayers) _array_element)
      (goto _label))))