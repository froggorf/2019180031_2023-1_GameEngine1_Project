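; BP_Ball is the ball actor for the baseball minigame, scoring for its assigned player and destroying itself five seconds after spawning.
; SetPlayerNumber stores the player index and swaps the sphere's material to match the first or second player.
; When the sphere begins overlapping a BP_CutLine, a DoOnce limits it to a single PlayerGetScore call on GM_BaseBall with that index.
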(event OnComponentBeginOverlap(Sphere)
  (params (OverlappedComponent :type Primitive%20Component%20Object%20Reference) (OtherActor :type Actor%20Object%20Reference) (OtherComp :type Primitive%20Component%20Object%20Reference) (OtherBodyIndex :type Integer) (bFromSweep :type Boolean) (SweepResult :type Hit%20Result%20Structure%20%28by%20ref%29))
  (Utilities|Casting|CastToBP_CutLine OtherActor)
  (Utilities|FlowControl|DoOnce false
    (:Completed
      (bind _asgm_base_ball (Utilities|Casting|CastToGM_BaseBall (Game|GetGameMode)))
      (Default|PlayerGetScore _asgm_base_ball (Variables|Default|GetPlayer%20Number)))))

(event Custom|Set%20Player%20Number
  (params (Player%20Number :type Integer))
  (bind _output_get (Variables|Default|SetPlayer%20Number Player%20Number))
  (switch int _output_get
    (:0
      (Rendering|Material|SetMaterial (Variables|Default|GetSphere) 0 "/Game/MiniGame/BaseBall/Character/MI_1stPlayer.MI_1stPlayer"))
    (:1
      (Rendering|Material|SetMaterial (Variables|Default|GetSphere) 0 "/Game/MiniGame/BaseBall/Character/MI_2ndPlayer.MI_2ndPlayer"))))

(event EventBeginPlay
  (Utilities|FlowControl|Delay 5.0)
  (Actor|DestroyActor))

(event Collision|EventActorBeginOverlap
  (params (OtherActor :type Actor%20Object%20Reference)))

(event EventTick
  (params (DeltaSeconds :type Float%20%28single-precision%29)))

(fn ConstructionScript)